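; BP_EnemyRookZ is an enemy rook unit that acquires a target through overlap and hands it to its AI controller, BP_EnemyRookControllerZ.
; When a BP_BaseUnit overlaps it, it writes that unit to the controller's NearestEnemy blackboard key, only if the key holds no valid object.
; BeginPlay, Tick and the construction script add no logic, and a node clearing hasTarget is left unconnected.
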(event EventBeginPlay
  (|CallParentFunction) ; This node is disabled and will not be called.\nDrag off pins to build functionality.
)

(event Collision|EventActorBeginOverlap
  (params (OtherActor :type Actor%20Object%20Reference))
  (bind _returnvalue (Utilities|Name|MakeLiteralName "NearestEnemy"))
  (bind _asbp_base_unit (Utilities|Casting|CastToBP_BaseUnit OtherActor))
  (bind _asbp_enemy_rook_controller_z (Utilities|Casting|CastToBP_EnemyRookControllerZ (Pawn|GetController (Variables|Default|GetTarget))))
  (if (Utilities|IsValid (AI|GetBlackboard _asbp_enemy_rook_controller_z))
    (Utilities|IsValid (AI|Components|Blackboard|GetValueasObject (AI|GetBlackboard _asbp_enemy_rook_controller_z) _returnvalue)
      (:Is%20Not%20Valid
        (AI|Components|Blackboard|SetValueasObject (AI|GetBlackboard _asbp_enemy_rook_controller_z) _returnvalue _asbp_base_unit)))))

(event EventTick
  (params (DeltaSeconds :type Float%20%28single-precision%29))
  (|CallParentFunction DeltaSeconds) ; This node is disabled and will not be called.\nDrag off pins to build functionality.
)

(fn ConstructionScript
  (|CallParentFunction))