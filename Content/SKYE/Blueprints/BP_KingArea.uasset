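; BP_KingArea is the visual area around a King, showing a colored ring and smoke for Heal, Speed or Damage stats.
; Construction creates a dynamic material on the mesh, which ChangeRingColor tints along with the decal.
; SR_ events forward ring and smoke changes to follow-up events, following a server-to-multicast naming pattern.
; The smoke event swaps the Niagara asset per stat, and SetTargetUnit stores the associated unit.
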(event Custom|SR_ChangeRing
  (params (col :type Color%20Structure))
  ;[1 1 1] change color of the ring
  (CallFunction|ChangeCol col))

(event Custom|changeCol
  (params (NewParam :type Color%20Structure))
  ;[1 1 1] change color of the ring
  (CallFunction|ChangeRingColor NewParam))

(event Custom|SR_ChangeSmoke
  (params (kingstat :type KingStatus%20Enum :default "NewEnumerator0"))
  (CallFunction|MCSmokeCol kingstat))

(event Custom|MC_SmokeCol
  (params (NewParam :type KingStatus%20Enum :default "NewEnumerator0"))
  (bind _smoke (Variables|Default|Getsmoke))
  (switch Utilities|FlowControl|Switch|SwitchonKingStatus NewParam
    (:NewEnumerator0
      (Class|NiagaraComponent|SetAsset _smoke "/Game/SKYE/Particles/UnitEffects/NS_KingAreaHeal.NS_KingAreaHeal" true))
    (:NewEnumerator1
      (Class|NiagaraComponent|SetAsset _smoke "/Game/SKYE/Particles/UnitEffects/NS_KingAreaSpeed.NS_KingAreaSpeed" true))
    (:NewEnumerator2
      (Class|NiagaraComponent|SetAsset _smoke "/Game/SKYE/Particles/UnitEffects/NS_KingAreaDamage.NS_KingAreaDamage" true))))

(fn ConstructionScript
  (bind _returnvalue (Rendering|Material|CreateDynamicMaterialInstance (Variables|Default|GetStaticMesh) 0 "/Game/SKYE/Materials/MI_KingArea.MI_KingArea" "None" :!class /Script/Engine.PrimitiveComponent))
  (Variables|Default|SetMat _returnvalue))

(fn SetTargetUnit
  (params (Unit :type Actor%20Object%20Reference))
  (Variables|Default|SetUnit Unit))

(fn ChangeRingColor
  (params (col :type Color%20Structure))
  (bind _returnvalue (Math|Conversions|ToLinearColor(Color) col))
  ;[1 1 1] change the color of the ring decal
  (Rendering|Material|SetVectorParameterValue (Variables|Default|GetMat) "BaseColor" _returnvalue :!class /Script/Engine.MaterialInstanceDynamic)
  (Rendering|Components|Decal|SetDecalColor (Variables|Default|GetDecal) _returnvalue))