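; BP_TileSpawnerSmall randomly generates a tile-based map on the server at BeginPlay.
; RandomGenBasicGrid walks a grid from Columns and Rows, spawning a random entry from Prefabs at each TileSpacing step.
; On outer indices 0 and 3, CheckIfBase leaves positions 0 to 3 empty for bases.
; An IsDarkTile flag toggles per outer iteration but does not affect spawning.
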(event Custom|SpawnMap
  ;[1 1 1] start the random generation of the map
  (CallFunction|RandomGenBasicGrid))

(event EventBeginPlay
  ;[1 1 1] start the random generation of the map
  (if (Networking|IsServer)
    (CallFunction|SpawnMap)))

(fn ConstructionScript)

(fn RandomGenBasicGrid
  (bind _tilespacing (Variables|Default|GetTileSpacing))
  ;[1 1 1] loop through columns and rows
  (for _index (range 0 (Variables|Default|GetColumns))
    (Variables|Default|SetIsDarkTile (not (Variables|Default|GetIsDarkTile)))
    (for _index_2 (range 0 (Variables|Default|GetRows))
      ;[1 1 1] If top or bottom row (where bases should be)
      (if (or (== _index 0) (== _index 3))
        (bind _isbase (CallFunction|CheckifBase _index_2))
        (if (not _isbase)
          ;[1 1 1] Spawn random tile at the next tile position
          (bind _output_get (Variables|Default|SetSpawnPos (Math|Vector|MakeVector (* _index_2 _tilespacing) (* _tilespacing _index) 0.0) :!label _label))
          (Game|SpawnActorfromClass (.OutItem (Utilities|Array|Random (Variables|Default|GetPrefabs))) (Math|Transform|MakeTransform _output_get "0, 0, 0" "1.000000,1.000000,1.000000") "Undefined" "MultiplyWithRoot" 0 0))
        (else
          (goto _label))))))

(fn CheckifBase
  (params (columIndex :type Integer))
  ;[1 1 1] If the middle tiles of the row where base should be
  (return (Math|Boolean|ORBoolean (== columIndex 0) (== columIndex 1) (== columIndex 2) (== columIndex 3))))