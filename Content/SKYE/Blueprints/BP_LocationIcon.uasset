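; BP_LocationIcon is a short-lived marker actor, apparently a location indicator, that spins and bobs, then destroys itself three seconds after BeginPlay.
; Each Tick rotates its static mesh and offsets it along local X, flipping direction when relative Z reaches a lower or upper limit.
; The motion uses fixed per-frame steps without delta-time scaling, so its speed depends on frame rate.
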(event EventBeginPlay
  ;[1 1 1] destroy self after 3 seconds
  (Utilities|FlowControl|Delay 3.0)
  (Actor|DestroyActor))

(event EventTick
  (params (DeltaSeconds :type Float%20%28single-precision%29))
  (bind _staticmesh (Variables|Default|GetStaticMesh))
  (bind _relativelocation (Variables|/Script/Engine.SceneComponent|GetRelativeLocation _staticmesh))
  ;[1 1 1] rotates and bobs up and down
  (Transformation|AddLocalRotation (Variables|Default|GetStaticMesh) "0.000000,0.000000,1.000000" false false)
  (if (<= (.z _relativelocation) 125.0)
    (Variables|Default|SetmoveAmount -0.75)
    (elif (>= (.z _relativelocation) 2e+02)
      (Variables|Default|SetmoveAmount 0.75)))
  (Transformation|AddLocalOffset (Variables|Default|GetStaticMesh) (Math|Vector|MakeVector (Variables|Default|GetmoveAmount) 0.0 0.0) false false))

(fn ConstructionScript)