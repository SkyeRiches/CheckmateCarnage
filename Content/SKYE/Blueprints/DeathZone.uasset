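; DeathZone is a box trigger that kills units that enter it by dealing massive damage through SRTakeDamage.
; On begin overlap it waits half a second, then casts the actor to friendly king, friendly rook or base unit.
; King and rook overlaps are filtered by component name, so the king's buff radius and the rook's range colliders do not trigger death.
; The single shared Delay ignores further overlaps while it counts down.
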(event OnComponentBeginOverlap(Box)
  (params (OverlappedComponent :type Primitive%20Component%20Object%20Reference) (OtherActor :type Actor%20Object%20Reference) (OtherComp :type Primitive%20Component%20Object%20Reference) (OtherBodyIndex :type Integer) (bFromSweep :type Boolean) (SweepResult :type Hit%20Result%20Structure%20%28by%20ref%29))
  (bind _returnvalue (Utilities|GetObjectName OtherComp))
  ;[1 1 1] kills any units that enter the death zone
  (Utilities|FlowControl|Delay 0.5)
  (bind _asmbp_friendly_king (Utilities|Casting|CastToMBP_FriendlyKing OtherActor)
    (:then
      (if (not (Utilities|Enum|Equal(Enum) (Utilities|GetObjectName OtherComp) "BuffRadius"))
        (Default|SRTakeDamage _asmbp_friendly_king 1e+03)))
    (:CastFailed
      (bind _asmbp_friendly_rook (Utilities|Casting|CastToMBP_FriendlyRook OtherActor)
        (:then
          (if (not (or (Utilities|Enum|Equal(Enum) _returnvalue "NorthSouthCollider") (Utilities|Enum|Equal(Enum) _returnvalue "EastWestCollider")))
            (Default|SRTakeDamage _asmbp_friendly_rook 1e+03)))
        (:CastFailed
          (bind _asmbp_base_unit (Utilities|Casting|CastToMBP_BaseUnit OtherActor))
          (Utilities|IsValid _asmbp_base_unit
            (:Is%20Valid
              (Default|SRTakeDamage _asmbp_base_unit 1e+03))))))))

(fn ConstructionScript)