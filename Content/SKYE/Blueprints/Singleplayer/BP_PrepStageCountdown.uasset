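; BP_PrepStageCountdown is an actor that times the singleplayer preparation stage before units become controllable.
; It starts on BeginPlay and decrements its timer every Tick.
; At zero it calls InitialiseAI on all enemy and unit controllers, then sets the player's RTS_Controller to allow unit control and leave the prep stage.
; It then deactivates itself if the controller cast succeeds.
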(event EventBeginPlay
  (Variables|Default|SetActivated true))

(event EventTick
  (params (DeltaSeconds :type Float%20%28single-precision%29))
  ;[1 1 1] counts down to zero then initialises ai and tells controller that units can now be controlled
  (if (Variables|Default|GetActivated)
    (Variables|Default|SetPrepStageTimer (- (Variables|Default|GetPrepStageTimer) DeltaSeconds))
    (if (<= (Variables|Default|GetPrepStageTimer) 0.0)
      (Utilities|FlowControl|Sequence
        (:then_0
          (bind _outactors (Actor|GetAllActorsOfClass "/Game/RORY/Singleplayer/Units/EnemyUnits/Blueprints/BP_BaseEnemyController.BP_BaseEnemyController_C"))
          (for _array_element _outactors
            (Default|InitialiseAI _array_element)))
        (:then_1
          (bind _outactors_2 (Actor|GetAllActorsOfClass "/Game/RORY/Singleplayer/Units/FriendlyUnits/FriendlyBPs/BP_BaseUnitController.BP_BaseUnitController_C"))
          (for _array_element_2 _outactors_2
            (Default|InitialiseAI _array_element_2)))
        (:then_2
          (bind _asrts_controller (Utilities|Casting|CastToRTS_Controller (Game|GetPlayerController 0)))
          (Variables|/Game/SKYE/Blueprints/Singleplayer/RTS_Controller.RTS_Controller_C|SetcanControlUnits _asrts_controller true)
          (Variables|/Game/SKYE/Blueprints/Singleplayer/RTS_Controller.RTS_Controller_C|SetinPrepStage _asrts_controller false))
        (:then_3
          (Variables|Default|SetActivated false))))))

(fn ConstructionScript)