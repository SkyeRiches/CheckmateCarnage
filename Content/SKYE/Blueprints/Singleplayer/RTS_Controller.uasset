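; RTS player controller for a single-player game with chess-piece units: selection, commands and budgeted unit placement.
; Enhanced Input drives click, Ctrl, drag-box and select-by-type selection, while Tick updates hover outlines, target rings and cursor.
; Right-click writes move or attack keys to each selected unit's AI blackboard, clearing prior orders.
; Placement multi-traces under the cursor for PlacementArea-tagged actors before spawning; refunds spare the King.
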(event Input|EnhancedActionEvents|EnhancedInputActionIA_Select
  (params (ActionValue :type Boolean) (ElapsedSeconds :type Float%20%28double-precision%29) (TriggeredSeconds :type Float%20%28double-precision%29) (InputAction :type Input%20Action%20Object%20Reference :default "/Game/SKYE/ControlScheme/IA_Select.IA_Select"))
  (bind _returnvalue (HUD|GetHUD))
  ;[1 1 1] Drag Select controls when click and drag
  (:Started
    (Utilities|Casting|CastToBP_BaseUnit (.hitactor (.HitResult (Game|Player|GetHitResultUnderCursorbyChannel (Game|GetPlayerController 0) "TraceTypeQuery2" true)))
      (:CastFailed
        (Class|SelectionInterface|StartSelection(Message) _returnvalue))))
  (:Completed
    (Class|SelectionInterface|StopSelection(Message) _returnvalue)))

(event Input|EnhancedActionEvents|EnhancedInputActionIA_Command
  (params (ActionValue :type Boolean) (ElapsedSeconds :type Float%20%28double-precision%29) (TriggeredSeconds :type Float%20%28double-precision%29) (InputAction :type Input%20Action%20Object%20Reference :default "/Game/SKYE/ControlScheme/IA_Command.IA_Command"))
  ;[1 1 1] Right Click action
  (:Started
    (if (Variables|Default|GetisHoldingUnitToPlace)
      (CallFunction|CancelUnitPlacement)
      (elif (Variables|Default|GetcanControlUnits)
        (CallFunction|CommandUnits)))))

(event Input|EnhancedActionEvents|EnhancedInputActionIA_SelectAll1
  (params (ActionValue :type Boolean) (ElapsedSeconds :type Float%20%28double-precision%29) (TriggeredSeconds :type Float%20%28double-precision%29) (InputAction :type Input%20Action%20Object%20Reference :default "/Game/SKYE/ControlScheme/IA_SelectAll1.IA_SelectAll1"))
  ;[1 1 1] 'Select all units of type' actions
  (:Started
    (if (Variables|Default|GetcanControlUnits)
      (CallFunction|SelectUnitsOfType "/Game/RORY/Singleplayer/Units/FriendlyUnits/FriendlyBPs/BP_FriendlyPawn.BP_FriendlyPawn_C"))))

(event Input|EnhancedActionEvents|EnhancedInputActionIA_SelectAll2
  (params (ActionValue :type Boolean) (ElapsedSeconds :type Float%20%28double-precision%29) (TriggeredSeconds :type Float%20%28double-precision%29) (InputAction :type Input%20Action%20Object%20Reference :default "/Game/SKYE/ControlScheme/IA_SelectAll2.IA_SelectAll2"))
  ;[1 1 1] 'Select all units of type' actions
  (if (Variables|Default|GetcanControlUnits)
    (CallFunction|SelectUnitsOfType "/Game/RORY/Singleplayer/Units/FriendlyUnits/FriendlyBPs/BP_FriendlyKnight.BP_FriendlyKnight_C")))

(event Input|EnhancedActionEvents|EnhancedInputActionIA_Select
  (params (ActionValue :type Boolean) (ElapsedSeconds :type Float%20%28double-precision%29) (TriggeredSeconds :type Float%20%28double-precision%29) (InputAction :type Input%20Action%20Object%20Reference :default "/Game/SKYE/ControlScheme/IA_Select.IA_Select"))
  ;[1 1 1] Left Click Action
  (:Started
    (if (Variables|Default|GetisHoldingUnitToPlace)
      (CallFunction|PlaceUnit)
      (else
        (CallFunction|SelectUnit)))))

(event Input|EnhancedActionEvents|EnhancedInputActionIA_SelectAll3
  (params (ActionValue :type Boolean) (ElapsedSeconds :type Float%20%28double-precision%29) (TriggeredSeconds :type Float%20%28double-precision%29) (InputAction :type Input%20Action%20Object%20Reference :default "/Game/SKYE/ControlScheme/IA_SelectAll3.IA_SelectAll3"))
  ;[1 1 1] 'Select all units of type' actions
  (if (Variables|Default|GetcanControlUnits)
    (CallFunction|SelectUnitsOfType "/Game/RORY/Singleplayer/Units/FriendlyUnits/FriendlyBPs/BP_FriendlyBishop.BP_FriendlyBishop_C")))

(event Input|EnhancedActionEvents|EnhancedInputActionIA_SelectAll4
  (params (ActionValue :type Boolean) (ElapsedSeconds :type Float%20%28double-precision%29) (TriggeredSeconds :type Float%20%28double-precision%29) (InputAction :type Input%20Action%20Object%20Reference :default "/Game/SKYE/ControlScheme/IA_SelectAll4.IA_SelectAll4"))
  ;[1 1 1] 'Select all units of type' actions
)

(event Input|EnhancedActionEvents|EnhancedInputActionIA_SelectAll5
  (params (ActionValue :type Boolean) (ElapsedSeconds :type Float%20%28double-precision%29) (TriggeredSeconds :type Float%20%28double-precision%29) (InputAction :type Input%20Action%20Object%20Reference :default "/Game/SKYE/ControlScheme/IA_SelectAll5.IA_SelectAll5"))
  ;[1 1 1] 'Select all units of type' actions
  (if (Variables|Default|GetcanControlUnits)
    (CallFunction|SelectUnitsOfType "/Game/RORY/Singleplayer/Units/FriendlyUnits/FriendlyBPs/BP_FriendlyQueen.BP_FriendlyQueen_C")))

(event Input|EnhancedActionEvents|EnhancedInputActionIA_SelectAll6
  (params (ActionValue :type Boolean) (ElapsedSeconds :type Float%20%28double-precision%29) (TriggeredSeconds :type Float%20%28double-precision%29) (InputAction :type Input%20Action%20Object%20Reference :default "/Game/SKYE/ControlScheme/IA_SelectAll6.IA_SelectAll6"))
  ;[1 1 1] 'Select all units of type' actions
  (if (Variables|Default|GetcanControlUnits)
    (CallFunction|SelectUnitsOfType "/Game/RORY/Singleplayer/Units/FriendlyUnits/FriendlyBPs/BP_FriendlyKing.BP_FriendlyKing_C")))

(event EventBeginPlay
  (bind _self self)
  (bind _returnvalue (PlayerController|LocalPlayerSubsystems|GetEnhancedInputLocalPlayerSubsystem _self))
  ;[1 1 1] Initialise the controller to use the new input system with the control scheme weve made
  (Utilities|IsValid _returnvalue
    (:Is%20Valid
      (Input|AddMappingContext _returnvalue "/Game/SKYE/ControlScheme/IMC_ControlScheme.IMC_ControlScheme" 0 "(bIgnoreAllPressedKeysUntilRelease=True,bForceImmediately=False,bNotifyUserSettings=False)")
      (Input|SetInputModeGameandUI _self 0 "LockAlways" false false)
      (Variables|Default|SetCurrentBudget 1000))))

(event EventTick
  (params (DeltaSeconds :type Float%20%28single-precision%29))
  ;[1 1 1] Update
  (if (Utilities|IsValid (Variables|Default|GetDragWidget))
    (bind _returnvalue (Class|WidgetLayoutLibrary|GetMousePositiononViewport))
    (Class|UserWidget|SetPositioninViewport (Variables|Default|GetDragWidget) (Math|Vector2D|MakeVector2D (- (.x (* _returnvalue (Class|WidgetLayoutLibrary|GetViewportScale))) 55.0) (- (.y (* _returnvalue (Class|WidgetLayoutLibrary|GetViewportScale))) 5e+01)) true))
  (if (Variables|Default|GetcanControlUnits)
    (CallFunction|HoverMouse)
    (if (Utilities|Array|IsNotEmpty (Variables|Default|GetSelectedUnit))
      (CallFunction|UpdateCursorImage)
      (else
        (Variables|/Script/Engine.PlayerController|SetCurrentMouseCursor (Game|GetPlayerController 0) "Default")))))

(fn ConstructionScript)

(fn SelectUnit
  (bind _returnvalue (Game|GetPlayerController 0))
  (bind (_hitresult _returnvalue_2) (Game|Player|GetHitResultUnderCursorbyChannel _returnvalue "TraceTypeQuery1" true))
  ;[1 1 1] Select the unit clicked on
  (if _returnvalue_2
    (bind _asbp_base_unit (Utilities|Casting|CastToBP_BaseUnit (.hitactor _hitresult))
      (:then
        (CallFunction|AddSelectedUnit _asbp_base_unit))
      (:CastFailed
        (CallFunction|SetUnitRingColor false)
        (Utilities|Array|Clear (Variables|Default|GetSelectedUnit))))))

(fn SetAttackTarget
  (params (EnemyTarget :type Object%20Object%20Reference) (Unit :type Actor%20Object%20Reference))
  ;[1 1 1] Set the attack target on the blackboard
  (AI|Components|Blackboard|SetValueasObject (AI|GetBlackboard Unit) (Utilities|Name|MakeLiteralName "Target") EnemyTarget))

(fn MoveUnit
  (params (Location :type Vector) (Unit :type Object%20Object%20Reference))
  ;[1 1 1] Set move pos on ai blackboard and then tell it to move
  (bind _asbp_base_unit (Utilities|Casting|CastToBP_BaseUnit Unit))
  (AI|Components|Blackboard|SetValueasVector (AI|GetBlackboard _asbp_base_unit) (Utilities|Name|MakeLiteralName "MovePos") Location)
  (AI|Components|Blackboard|SetValueasBool (AI|GetBlackboard _asbp_base_unit) (Utilities|Name|MakeLiteralName "hasMovePos") true)
  (AI|Components|Blackboard|SetValueasBool (AI|GetBlackboard _asbp_base_unit) (Utilities|Name|MakeLiteralName "hasTarget") false))

(fn ClearUnitInstructions
  (params (Unit :type Actor%20Object%20Reference))
  (bind _returnvalue (AI|GetBlackboard Unit))
  ;[1 1 1] set blackboard values as empty/false, this will make the behaviour tree abort whatever behaviour its currently doing
  (AI|Components|Blackboard|SetValueasBool _returnvalue (Utilities|Name|MakeLiteralName "Attacking") false)
  (AI|Components|Blackboard|SetValueasObject _returnvalue (Utilities|Name|MakeLiteralName "Target") 0)
  (AI|Components|Blackboard|SetValueasBool _returnvalue (Utilities|Name|MakeLiteralName "Moving") false))

(fn AddSelectedUnit
  (params (Unit :type Actor%20Object%20Reference))
  ;[0.2708 0.2708 0.2708] Add unit clicked on to array of selected units
  (if (Utilities|IsValid Unit)
    (if (Utilities|Array|ContainsItem (Variables|Default|GetSelectedUnit) Unit) ; if item is already selected
      (if (Input|EnhancedActionValues|GetIA_ctrl) ; if holding ctr and clicking on unit already selected,\ndeselect it
        ;;[1 1 1] Deselect item
        (bind _asbp_base_unit (Utilities|Casting|CastToBP_BaseUnit Unit :!label _label))
        (Default|RingDefaultColor _asbp_base_unit)
        (Utilities|Array|RemoveItem (Variables|Default|GetSelectedUnit) Unit)
        (elif (< (Utilities|Array|Length (Variables|Default|GetSelectedUnit)) 2) ; if there is only one selected and you click on it\ndeselect it\nif there is more than one, select only that one
          (goto _label)
          (else
            ;;[1 1 1] Overwrite currently selected
            (CallFunction|SetUnitRingColor false :!label _label_2)
            (Utilities|Array|Clear (Variables|Default|GetSelectedUnit)) ; if not holding control, overwrite list
            (Utilities|Array|AddUnique (Variables|Default|GetSelectedUnit) Unit :!label _label_3)
            (CallFunction|SetUnitRingColor true))))
      (elif (Input|EnhancedActionValues|GetIA_ctrl)
        (goto _label_3)
        (else
          (goto _label_2))))))

(fn SetUnitRingColor
  (params (isSelected :type Boolean))
  ;[1 1 1] sets the color of the ring around the unit based on whether they are selected or not
  (for _array_element (Variables|Default|GetSelectedUnit)
    (bind _asbp_base_unit (Utilities|Casting|CastToBP_BaseUnit _array_element))
    (if (Utilities|IsValid _asbp_base_unit)
      (if isSelected
        (Default|RingSelectColor _asbp_base_unit)
        (else
          (Default|RingDefaultColor _asbp_base_unit))))))

(fn DragSelect
  (params (Selected :type Array%20of%20Actor%20Object%20References))
  (LocalVariables|SetSelectedByDrag Selected)
  ;[1 1 1] If not enemy, add it to the list of selected units
  (for _array_element (LocalVariables|GetSelectedByDrag)
    (bind _asbp_base_unit (Utilities|Casting|CastToBP_BaseUnit _array_element))
    (Utilities|Array|AddUnique (Variables|Default|GetSelectedUnit) _asbp_base_unit)
    (Default|RingSelectColor _asbp_base_unit))
  ;[1 1 1] If when dragging, the unit is no longer encompassed by the selection square, deselect it
  (for _array_element_2 (Variables|Default|GetSelectedUnit)
    (if (not (Utilities|Array|ContainsItem (LocalVariables|GetSelectedByDrag) _array_element_2))
      (bind _asbp_base_unit_2 (Utilities|Casting|CastToBP_BaseUnit _array_element_2))
      (Default|RingDefaultColor _asbp_base_unit_2)
      (Utilities|Array|RemoveItem (Variables|Default|GetSelectedUnit) _asbp_base_unit_2))))

(fn CommandUnits
  (bind _returnvalue (Game|GetPlayerController 0))
  (bind _hitresult (Game|Player|GetHitResultUnderCursorbyChannel _returnvalue "TraceTypeQuery2" true))
  (bind _asbp_base_enemy (Utilities|Casting|CastToBP_BaseEnemy (.hitactor _hitresult))
    (:then
      (if true
        ;[1 1 1] Attack Command
        (for _array_element (Variables|Default|GetSelectedUnit)
          (if (Utilities|IsValid _array_element)
            (CallFunction|ClearUnitInstructions _array_element) ; should interrupt any other command
            (if (Utilities|IsValid _asbp_base_enemy)
              (CallFunction|MovetoAttack (Transformation|GetActorLocation _asbp_base_enemy) _array_element)
              (CallFunction|SetAttackTarget _asbp_base_enemy _array_element))
            (else
              (Utilities|Array|RemoveItem (Variables|Default|GetSelectedUnit) _array_element) ; if the item isnt valid, remove it from the array so it doesnt try to use that item again
            )))))
    (:CastFailed
      (if (not (Utilities|Array|IsEmpty (Variables|Default|GetSelectedUnit)))
        ;[1 1 1] Move Command
        (CallFunction|PlaceRing (.impactpoint _hitresult))
        (for _array_element_2 (Variables|Default|GetSelectedUnit)
          (CallFunction|ClearUnitInstructions _array_element_2) ; should interrupt any other command
          (CallFunction|MoveUnit (.impactpoint _hitresult) _array_element_2))))))

(fn PlaceRing
  (params (Location :type Vector))
  ;[1 1 1] spawns the ring at the move location so you can see where the unit will move to
  (if (Utilities|IsValid (Variables|Default|GetLocationRing))
    (Actor|DestroyActor (Variables|Default|GetLocationRing)))
  (bind _returnvalue (Game|SpawnActorfromClass "/Game/SKYE/Blueprints/BP_LocationIcon.BP_LocationIcon_C" (Math|Transform|MakeTransform Location "0, 0, 0" "1.000000,1.000000,1.000000") "Undefined" "MultiplyWithRoot" 0 0))
  (Variables|Default|SetLocationRing _returnvalue))

(fn HoverMouse
  (bind _returnvalue (Game|GetPlayerController 0))
  (bind _hitresult (Game|Player|GetHitResultUnderCursorbyChannel _returnvalue "TraceTypeQuery2" true))
  (CallFunction|ClearHighlight)
  (bind _asbp_base_unit (Utilities|Casting|CastToBP_BaseUnit (.hitactor _hitresult))
    (:then
      ;[1 1 1] If its not an enemy unit, highlight blue if not selected, or highlight white if selected and disable any target rings on enemies that might be active
      (if (Utilities|Array|ContainsItem (Variables|Default|GetSelectedUnit) _asbp_base_unit)
        (Default|HighlightUnit _asbp_base_unit)
        (else
          (Default|HighlightUnit _asbp_base_unit 1)))
      (Variables|Default|SetHighlightedFriend _asbp_base_unit)
      (if (Utilities|IsValid (Variables|Default|GetHighlightedEnemy))
        (Default|HideTargetRing (Variables|Default|GetHighlightedEnemy))
        (Variables|Default|SetHighlightedEnemy 0)))
    (:CastFailed
      (bind _asbp_base_enemy (Utilities|Casting|CastToBP_BaseEnemy (.hitactor _hitresult)))
      ;[1 1 1] If hovering over enemy, show the target ring and hightlight them with the red outline
      (if (Utilities|Array|IsNotEmpty (Variables|Default|GetSelectedUnit))
        (Default|ShowTargetRing _asbp_base_enemy))
      (Default|HighlightUnit _asbp_base_enemy 2)
      (Variables|Default|SetHighlightedEnemy _asbp_base_enemy))))

(fn ClearHighlight
  ;[1 1 1] Disables the outline highlight of the object
  (if (Utilities|IsValid (Variables|Default|GetHighlightedEnemy)) ; whether its a friendly unit that was\nhoevered on or if it was enemy
    (Default|HideTargetRing (Variables|Default|GetHighlightedEnemy))
    (Default|UnHighlightUnit (Variables|Default|GetHighlightedEnemy))
    (Variables|Default|SetHighlightedEnemy 0) ; reset highlighted enemy
  )
  (if (Utilities|IsValid (Variables|Default|GetHighlightedFriend))
    (Default|UnHighlightUnit (Variables|Default|GetHighlightedFriend))
    (Variables|Default|SetHighlightedFriend 0) ; reset highlighted friend
  ))

(fn MovetoAttack
  (params (Location :type Vector) (Unit :type Object%20Object%20Reference))
  ;[1 1 1] Set move pos on ai blackboard and then tell it to move
  (bind _asbp_base_unit (Utilities|Casting|CastToBP_BaseUnit Unit))
  (AI|Components|Blackboard|SetValueasVector (AI|GetBlackboard _asbp_base_unit) (Utilities|Name|MakeLiteralName "MovePos") Location)
  (AI|Components|Blackboard|SetValueasBool (AI|GetBlackboard _asbp_base_unit) (Utilities|Name|MakeLiteralName "hasTarget") true)
  (AI|Components|Blackboard|SetValueasBool (AI|GetBlackboard _asbp_base_unit) (Utilities|Name|MakeLiteralName "hasMovePos") false))

(fn IncreaseBudget
  (params (Amount :type Integer))
  (Variables|Default|SetCurrentBudget (+ (Variables|Default|GetCurrentBudget) Amount)))

(fn ReduceBudget
  (params (Amount :type Integer))
  (Variables|Default|SetCurrentBudget (- (Variables|Default|GetCurrentBudget) Amount)))

(fn SelectUnitsOfType
  (params (UnitType :type Actor%20Class%20Reference))
  ;[1 1 1] find all units of specified type and add them to selected units. if selected units contains anything, clear it first
  (if (Utilities|Array|IsEmpty (Variables|Default|GetSelectedUnit))
    (bind _outactors (Actor|GetAllActorsOfClass UnitType))
    (for _array_element _outactors
      (Utilities|Array|AddUnique (Variables|Default|GetSelectedUnit) _array_element))
    (CallFunction|SetUnitRingColor true)
    (else
      (CallFunction|SetUnitRingColor false)
      (Utilities|Array|Clear (Variables|Default|GetSelectedUnit))
      (bind _outactors_2 (Actor|GetAllActorsOfClass UnitType))
      (for _array_element_2 _outactors_2
        (Utilities|Array|AddUnique (Variables|Default|GetSelectedUnit) _array_element_2))
      (CallFunction|SetUnitRingColor true))))

(fn UpdateCursorImage
  (bind _hitresult (Game|Player|GetHitResultUnderCursorbyChannel "TraceTypeQuery1" true))
  (bind _returnvalue (Game|GetPlayerController 0))
  ;[1 1 1] change cursor image depending on what mouse is hovering on
  (Utilities|Casting|CastToBP_BaseEnemy (.hitactor _hitresult)
    (:then
      (Variables|/Script/Engine.PlayerController|SetCurrentMouseCursor (Game|GetPlayerController 0) "Crosshairs") ; attack cursor
    )
    (:CastFailed
      (Utilities|Casting|CastToBP_BaseUnit (.hitactor _hitresult)
        (:then
          (Variables|/Script/Engine.PlayerController|SetCurrentMouseCursor _returnvalue "Default"))
        (:CastFailed
          (Variables|/Script/Engine.PlayerController|SetCurrentMouseCursor _returnvalue "Hand") ; move action cursor
        )))))

(fn PlaceUnit
  ;[1 1 1] check if have enough budget, then fire multiple rays, check for placement area, if in placement area, spawn unit and reduce budget
  (LocalVariables|SetInPlacementArea false)
  (if (>= (- (Variables|Default|GetCurrentBudget) (Variables|Default|GetUnitCost)) 0)
    (bind _returnvalue (Class|WidgetLayoutLibrary|GetMousePositiononViewport))
    (bind _outhits (Collision|MultiLineTraceByChannel (.WorldPosition (Class|GameplayStatics|DeprojectScreentoWorld self (* _returnvalue (Class|WidgetLayoutLibrary|GetViewportScale)))) (+ (.WorldPosition (Class|GameplayStatics|DeprojectScreentoWorld self (* _returnvalue (Class|WidgetLayoutLibrary|GetViewportScale)))) (* (.WorldDirection (Class|GameplayStatics|DeprojectScreentoWorld self (* _returnvalue (Class|WidgetLayoutLibrary|GetViewportScale)))) (LocalVariables|GetRayLength))) "TraceTypeQuery1" false 0 "None"))
    (for _array_element _outhits
      (if (.bBlockingHit (Collision|BreakHitResult _array_element))
        (if (LocalVariables|GetInPlacementArea)
          (Game|SpawnActorfromClass (Variables|Default|GetUnitType) (Math|Transform|MakeTransform (+ (.Location (Collision|BreakHitResult _array_element)) "0.000000,0.000000,110.000000") "0, 0, 0" "1.000000,1.000000,1.000000") "AlwaysSpawn" "MultiplyWithRoot" 0 0)
          (CallFunction|ReduceBudget (Variables|Default|GetUnitCost))
          (return))
        (elif (Actor|ActorHasTag (.HitActor (Collision|BreakHitResult _array_element)) "PlacementArea")
          (LocalVariables|SetInPlacementArea true))))))

(fn StoreUnittoPlace
  (params (Type :type Actor%20Class%20Reference) (Cost :type Integer) (Widget :type Drag%20Widget%20Object%20Reference))
  ;[1 1 1] stores info about the click and place system
  (Variables|Default|SetUnitType Type)
  (Variables|Default|SetUnitCost Cost)
  (Variables|Default|SetDragWidget Widget)
  (Variables|Default|SetisHoldingUnitToPlace true))

(fn CancelUnitPlacement
  ;[1 1 1] remove info on the unit that was being held to place
  (Variables|Default|SetisHoldingUnitToPlace false)
  (Variables|Default|SetDragWidget 0)
  (Variables|Default|SetUnitType 0)
  (Variables|Default|SetUnitCost 0))

(fn RefundUnit
  ;[1 1 1] increase budget by unit cost and delete unit
  (for _array_element (Variables|Default|GetSelectedUnit)
    (Utilities|Casting|CastToBP_FriendlyKing _array_element
      (:CastFailed
        (bind _asbp_base_unit (Utilities|Casting|CastToBP_BaseUnit _array_element))
        (Variables|Default|SetCurrentBudget (+ (Variables|/Game/RORY/Singleplayer/Units/FriendlyUnits/FriendlyBPs/BP_BaseUnit.BP_BaseUnit_C|GetCost _asbp_base_unit) (Variables|Default|GetCurrentBudget)))
        (if (Utilities|IsValid (Variables|/Script/AIModule.AIController|GetBrainComponent (AI|GetAIController _asbp_base_unit)))
          (AI|Logic|StopLogic (Variables|/Script/AIModule.AIController|GetBrainComponent (AI|GetAIController _asbp_base_unit)) ""))
        (Actor|DestroyActor (AI|GetAIController _asbp_base_unit))
        (Actor|DestroyActor _asbp_base_unit)))))