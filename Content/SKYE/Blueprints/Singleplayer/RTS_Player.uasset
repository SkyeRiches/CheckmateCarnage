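; RTS camera pawn for the player, which also toggles the pause menu.
; Enhanced Input drives keyboard movement, middle-mouse panning, yaw, spring-arm pitch and curve-mapped zoom.
; When not panning, Tick clamps the position to map bounds and edge-scrolls faster toward screen edges unless RTS_Controller blocks it, using that controller's speed and margin.
; Pausing sets global time dilation to zero and disables unit control, which unpausing restores outside the prep stage.
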(event Input|EnhancedActionEvents|EnhancedInputActionIA_MoveVertical
  (params (ActionValue :type Float%20%28double-precision%29) (ElapsedSeconds :type Float%20%28double-precision%29) (TriggeredSeconds :type Float%20%28double-precision%29) (InputAction :type Input%20Action%20Object%20Reference :default "/Game/SKYE/ControlScheme/IA_MoveVertical.IA_MoveVertical"))
  ;[1 1 1] Keyboard controls for movement
  (CallFunction|WSMove ActionValue))

(event Input|EnhancedActionEvents|EnhancedInputActionIA_MoveHorizontal
  (params (ActionValue :type Float%20%28double-precision%29) (ElapsedSeconds :type Float%20%28double-precision%29) (TriggeredSeconds :type Float%20%28double-precision%29) (InputAction :type Input%20Action%20Object%20Reference :default "/Game/SKYE/ControlScheme/IA_MoveHorizontal.IA_MoveHorizontal"))
  ;[1 1 1] Keyboard controls for movement
  (CallFunction|ADMove ActionValue))

(event Input|EnhancedActionEvents|EnhancedInputActionIA_Zoom
  (params (ActionValue :type Float%20%28double-precision%29) (ElapsedSeconds :type Float%20%28double-precision%29) (TriggeredSeconds :type Float%20%28double-precision%29) (InputAction :type Input%20Action%20Object%20Reference :default "/Game/SKYE/ControlScheme/IA_Zoom.IA_Zoom"))
  ;[1 1 1] Move the camera closer or futher
  (CallFunction|Zoom ActionValue))

(event Input|EnhancedActionEvents|EnhancedInputActionIA_RotateCamera
  (params (ActionValue :type Float%20%28double-precision%29) (ElapsedSeconds :type Float%20%28double-precision%29) (TriggeredSeconds :type Float%20%28double-precision%29) (InputAction :type Input%20Action%20Object%20Reference :default "/Game/SKYE/ControlScheme/IA_RotateCamera.IA_RotateCamera"))
  ;[1 1 1] Rotate camera left and right and up and down
  (CallFunction|RotateView ActionValue))

(event Input|EnhancedActionEvents|EnhancedInputActionIA_PitchCamera
  (params (ActionValue :type Float%20%28double-precision%29) (ElapsedSeconds :type Float%20%28double-precision%29) (TriggeredSeconds :type Float%20%28double-precision%29) (InputAction :type Input%20Action%20Object%20Reference :default "/Game/SKYE/ControlScheme/IA_PitchCamera.IA_PitchCamera"))
  ;[1 1 1] Rotate camera left and right and up and down
  (CallFunction|PitchCamera ActionValue))

(event Input|EnhancedActionEvents|EnhancedInputActionIA_MiddleClick
  (params (ActionValue :type Boolean) (ElapsedSeconds :type Float%20%28double-precision%29) (TriggeredSeconds :type Float%20%28double-precision%29) (InputAction :type Input%20Action%20Object%20Reference :default "/Game/SKYE/ControlScheme/IA_MiddleClick.IA_MiddleClick"))
  ;[1 1 1] Move the camera by holding middle click and moving mouse
  (:Triggered
    (Variables|Default|SetisPanning true)
    (CallFunction|PanCamera))
  (:Canceled
    (Variables|Default|SetisPanning false :!label _label))
  (:Completed
    (goto _label)))

(event Input|EnhancedActionEvents|EnhancedInputActionIA_PauseMenu
  (params (ActionValue :type Boolean) (ElapsedSeconds :type Float%20%28double-precision%29) (TriggeredSeconds :type Float%20%28double-precision%29) (InputAction :type Input%20Action%20Object%20Reference :default "/Game/SKYE/ControlScheme/IA_PauseMenu.IA_PauseMenu"))
  (bind _returnvalue (Game|GetPlayerController 0))
  ;[1 1 1] Pause menu
  (:Started
    (if (Variables|Default|GetisPaused)
      (Utilities|FlowControl|Sequence
        (:then_0
          (bind _foundwidgets (Widget|GetAllWidgetsOfClass "/Game/SKYE/Blueprints/Singleplayer/UI/WB_OptionsMenu.WB_OptionsMenu_C" true))
          (for _array_element _foundwidgets
            (Widget|RemovefromParent _array_element)))
        (:then_1
          (bind _foundwidgets_2 (Widget|GetAllWidgetsOfClass "/Game/SKYE/Blueprints/Singleplayer/UI/WB_ControlPage.WB_ControlPage_C" true))
          (for _array_element_2 _foundwidgets_2
            (Widget|RemovefromParent _array_element_2)))
        (:then_2
          (Variables|Default|SetisPaused false)
          (Widget|RemovefromParent (Variables|Default|GetPauseMenu))
          (Utilities|Time|SetGlobalTimeDilation 1.0)
          (bind _asrts_controller (Utilities|Casting|CastToRTS_Controller _returnvalue))
          (if (not (Variables|/Game/SKYE/Blueprints/Singleplayer/RTS_Controller.RTS_Controller_C|GetinPrepStage _asrts_controller))
            (Variables|/Game/SKYE/Blueprints/Singleplayer/RTS_Controller.RTS_Controller_C|SetcanControlUnits _asrts_controller true))))
      (else
        (bind _returnvalue_2 (UserInterface|CreateWidget "/Game/SKYE/Blueprints/Singleplayer/UI/WB_PauseMenu.WB_PauseMenu_C"))
        (UserInterface|Viewport|AddtoViewport _returnvalue_2 0)
        (Variables|Default|SetPauseMenu _returnvalue_2)
        (Variables|Default|SetisPaused true)
        (Utilities|Time|SetGlobalTimeDilation 0.0)
        (bind _asrts_controller_2 (Utilities|Casting|CastToRTS_Controller _returnvalue))
        (Variables|/Game/SKYE/Blueprints/Singleplayer/RTS_Controller.RTS_Controller_C|SetcanControlUnits _asrts_controller_2 false)))))

(event EventBeginPlay
  ;[1 1 1] Initialise it to use the camera as the view
  (Game|Player|SetViewTargetwithBlend (Game|GetPlayerController 0) self 0.0 "VTBlend_Linear" 0.0 false)
  ;[1 1 1] intialise camera zoom and rotation
  (CallFunction|Zoom 0.0)
  (Transformation|SetRelativeRotation (Variables|Default|GetSpringArm) (Math|Rotator|MakeRotator 0.0 -45.0 9e+01) false false)
  (bind _asrts_controller (Utilities|Casting|CastToRTS_Controller (Game|GetPlayerController 0)))
  (Variables|Default|SetRTSController _asrts_controller))

(event EventTick
  (params (DeltaSeconds :type Float%20%28single-precision%29))
  ;[1 1 1] the bounds movement system, called on update
  (if (not (Variables|Default|GetisPanning))
    (if (Variables|/Game/SKYE/Blueprints/Singleplayer/RTS_Controller.RTS_Controller_C|GetDontMoveMouse (Variables|Default|GetRTSController))
      _
      (else
        (CallFunction|MoveLeft)
        (CallFunction|MoveRight)
        (CallFunction|MoveUp)
        (CallFunction|MoveDown)))
    (CallFunction|ClampMovement)))

(fn ConstructionScript)

(fn MoveLeft
  ;[1 1 1] Moves the camera left
  (bind _returnvalue (Class|WidgetLayoutLibrary|GetMousePositiononViewport))
  (Transformation|AddActorLocalOffset (* (* (* (Math|Vector|MakeVector (Variables|/Game/SKYE/Blueprints/Singleplayer/RTS_Controller.RTS_Controller_C|GetSpeed (Variables|Default|GetRTSController)) 0.0 0.0) (- 1.0 (Math|Float|Clamp(Float) (Math|Float|NormalizetoRange (.x (* _returnvalue (Class|WidgetLayoutLibrary|GetViewportScale))) 0.0 (* (.x (Viewport|GetViewportSize)) (Variables|/Game/SKYE/Blueprints/Singleplayer/RTS_Controller.RTS_Controller_C|GetEdgeMargin (Variables|Default|GetRTSController))))))) (Utilities|Time|GetWorldDeltaSeconds)) 6e+01) false false))

(fn MoveRight
  (bind _returnvalue (Viewport|GetViewportSize))
  ;[1 1 1] moves then camera right
  (bind _returnvalue_2 (Class|WidgetLayoutLibrary|GetMousePositiononViewport))
  (Transformation|AddActorLocalOffset (* (* (* (Math|Vector|MakeVector (* (Variables|/Game/SKYE/Blueprints/Singleplayer/RTS_Controller.RTS_Controller_C|GetSpeed (Variables|Default|GetRTSController)) -1.0) 0.0 0.0) (Math|Float|Clamp(Float) (Math|Float|NormalizetoRange (.x (* _returnvalue_2 (Class|WidgetLayoutLibrary|GetViewportScale))) (* (.x _returnvalue) (- 1.0 (Variables|/Game/SKYE/Blueprints/Singleplayer/RTS_Controller.RTS_Controller_C|GetEdgeMargin (Variables|Default|GetRTSController)))) (.x _returnvalue)))) (Utilities|Time|GetWorldDeltaSeconds)) 6e+01) false false))

(fn MoveUp
  ;[1 1 1] move camera up
  (bind _returnvalue (Class|WidgetLayoutLibrary|GetMousePositiononViewport))
  (Transformation|AddActorLocalOffset (* (* (* (Math|Vector|MakeVector 0.0 (Variables|/Game/SKYE/Blueprints/Singleplayer/RTS_Controller.RTS_Controller_C|GetSpeed (Variables|Default|GetRTSController)) 0.0) (- 1.0 (Math|Float|Clamp(Float) (Math|Float|NormalizetoRange (.y (* _returnvalue (Class|WidgetLayoutLibrary|GetViewportScale))) 0.0 (* (.y (Viewport|GetViewportSize)) (Variables|/Game/SKYE/Blueprints/Singleplayer/RTS_Controller.RTS_Controller_C|GetEdgeMargin (Variables|Default|GetRTSController))))))) (Utilities|Time|GetWorldDeltaSeconds)) 6e+01) false false))

(fn MoveDown
  (bind _returnvalue (Viewport|GetViewportSize))
  ;[1 1 1] move camera down
  (bind _returnvalue_2 (Class|WidgetLayoutLibrary|GetMousePositiononViewport))
  (Transformation|AddActorLocalOffset (* (* (* (Math|Vector|MakeVector 0.0 (* (Variables|/Game/SKYE/Blueprints/Singleplayer/RTS_Controller.RTS_Controller_C|GetSpeed (Variables|Default|GetRTSController)) -1.0) 0.0) (Math|Float|Clamp(Float) (Math|Float|NormalizetoRange (.y (* _returnvalue_2 (Class|WidgetLayoutLibrary|GetViewportScale))) (* (.y _returnvalue) (- 1.0 (Variables|/Game/SKYE/Blueprints/Singleplayer/RTS_Controller.RTS_Controller_C|GetEdgeMargin (Variables|Default|GetRTSController)))) (.y _returnvalue)))) (Utilities|Time|GetWorldDeltaSeconds)) 6e+01) false false))

(fn WSMove
  (params (Input :type Float%20%28double-precision%29))
  ;[1 1 1] move camera forward and back with ws
  (Transformation|AddActorLocalOffset (* (* (* (Math|Vector|MakeVector 0.0 (Variables|/Game/SKYE/Blueprints/Singleplayer/RTS_Controller.RTS_Controller_C|GetSpeed (Variables|Default|GetRTSController)) 0.0) Input) (Utilities|Time|GetWorldDeltaSeconds)) 6e+01) false false))

(fn ADMove
  (params (Input :type Float%20%28double-precision%29))
  ;[1 1 1] move camera left and right
  (Transformation|AddActorLocalOffset (* (* (* (Math|Vector|MakeVector (Variables|/Game/SKYE/Blueprints/Singleplayer/RTS_Controller.RTS_Controller_C|GetSpeed (Variables|Default|GetRTSController)) 0.0 0.0) Input) (Utilities|Time|GetWorldDeltaSeconds)) 6e+01) false false))

(fn Zoom
  (params (Input :type Float%20%28double-precision%29))
  (bind _curve (Variables|Default|GetCurve))
  (bind (_mintime _maxtime) (Math|Curves|GetTimeRange _curve))
  ;[1 1 1] Scroll to move the camera closer or further on the spring arm (acts as a zoom)
  (Variables|Default|SetScrollValue (Math|Float|Clamp(Float) (+ (Variables|Default|GetScrollValue) (* (* Input -1.0) (Variables|Default|GetScrollSpeed))) _mintime _maxtime))
  (Variables|/Script/Engine.SpringArmComponent|SetTargetArmLength (Variables|Default|GetSpringArm) (* (Math|Curves|GetFloatValue (Variables|Default|GetCurve) (Variables|Default|GetScrollValue)) 1e+03)))

(fn RotateView
  (params (Input :type Float%20%28double-precision%29))
  (bind _self self)
  ;[1 1 1] rotate camera left and right with qe
  (Transformation|SetActorRotation _self (Math|Rotator|MakeRotator 0.0 0.0 (+ (* Input (Variables|Default|GetRotateSpeed)) (.yaw (Transformation|GetActorRotation _self))))))

(fn ClampMovement
  (bind _returnvalue (Transformation|GetActorLocation))
  (bind _boundsmin (Variables|Default|GetBoundsMin))
  (bind _boundsmax (Variables|Default|GetBoundsMax))
  ;[1 1 1] stop the camera from moving beyond the bounds of the map
  (Transformation|SetActorLocation (Math|Vector|MakeVector (Math|Float|Clamp(Float) (.x _returnvalue) (.x _boundsmin) (.x _boundsmax)) (Math|Float|Clamp(Float) (.y _returnvalue) (.y _boundsmin) (.y _boundsmax)) (.z _returnvalue)) false false))

(fn PitchCamera
  (params (Input :type Float%20%28double-precision%29))
  (bind _springarm (Variables|Default|GetSpringArm))
  ;[1 1 1] Rotate camera along y access to make it point up and down
  (Transformation|SetRelativeRotation _springarm (Math|Rotator|MakeRotator 0.0 (Math|Float|Clamp(Float) (+ (* Input (Variables|Default|GetRotateSpeed)) (.pitch (Class|SpringArmComponent|GetTargetRotation _springarm))) -9e+01 -2e+01) 9e+01) false false))

(fn PanCamera
  ;[1 1 1] Move the camera
  (Transformation|AddActorLocalOffset (* (* (* (Input|EnhancedActionValues|GetIA_MousePos) (+ (Variables|/Game/SKYE/Blueprints/Singleplayer/RTS_Controller.RTS_Controller_C|GetSpeed (Variables|Default|GetRTSController)) 5e+01)) (Utilities|Time|GetWorldDeltaSeconds)) 6e+01) false false))