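; Multiplayer game mode for an RTS match that tracks connected MRTS_Controllers and copies each player's team from the game instance on controller swap.
; It spawns player pawns, kings and units at team-tagged player starts or given locations, facing by team.
; BeginGame activates unit AI and unlocks control after the prep stage.
; Endgame and DrawGame freeze time via global dilation and show each player the result.
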(event Custom|stoptime
  ;[1 1 1] stop time for everyone (called at end of game)
  (Utilities|Time|SetGlobalTimeDilation 0.0))

(event EventPostLogin
  (params (NewPlayer :type Player%20Controller%20Object%20Reference))
  ;[1 1 1] events for when player connnects
  (bind _asmrts_controller (Utilities|Casting|CastToMRTS_Controller NewPlayer))
  (Utilities|Array|AddUnique (Variables|Default|GetPlayers) _asmrts_controller))

(event EventOnSwapPlayerControllers
  (params (OldPC :type Player%20Controller%20Object%20Reference) (NewPC :type Player%20Controller%20Object%20Reference))
  ;[1 1 1] events for when player connnects
  (bind _asmrts_controller (Utilities|Casting|CastToMRTS_Controller NewPC))
  (Utilities|Array|AddUnique (Variables|Default|GetPlayers) _asmrts_controller)
  (bind _asps_multiplayer (Utilities|Casting|CastToPS_Multiplayer (Variables|/Script/Engine.Controller|GetPlayerState _asmrts_controller)))
  (bind _asgi_checkmate_carnage_steam (Utilities|Casting|CastToGI_CheckmateCarnageSteam (Game|GetGameInstance)))
  (Variables|/Game/SKYE/Blueprints/Multiplayer/Networking/Blueprints/PS_Multiplayer.PS_Multiplayer_C|SetTeam _asps_multiplayer (Variables|/Game/SKYE/Blueprints/Multiplayer/Networking/Blueprints/GI_CheckmateCarnageSteam.GI_CheckmateCarnageSteam_C|GetTeam _asgi_checkmate_carnage_steam)))

(event EventOnLogout
  (params (ExitingController :type Controller%20Object%20Reference))
  ;[1 1 1] player disconnects
  (bind _asmrts_controller (Utilities|Casting|CastToMRTS_Controller ExitingController))
  (Utilities|Array|RemoveItem (Variables|Default|GetPlayers) _asmrts_controller))

(fn ConstructionScript)

(fn FindTeamPlayerStart
  (params (team :type Name))
  ;[1 1 1] find the start position for the specified team
  (bind _outactors (Actor|GetAllActorsOfClass "/Script/Engine.PlayerStart"))
  (for _array_element _outactors
    (if (Actor|ActorHasTag _array_element team)
      (return (Transformation|GetActorTransform _array_element)))))

(fn SpawnPlayer
  (params (PlayerState :type PS%20Multiplayer%20Object%20Reference) (PlayerController :type MRTS%20Controller%20Object%20Reference) (team :type Team%20Enum :default "NewEnumerator0"))
  (bind _returnvalue (Pawn|GetControlledPawn PlayerController))
  ;[1 1 1] spawn new player
  (Utilities|IsValid _returnvalue
    (:Is%20Valid
      (Actor|DestroyActor _returnvalue) ; to be safe, if one exists, delete it and spawn a new
    )
    (:Is%20Not%20Valid
      _))
  (bind _returnvalue_2 (Game|SpawnActorfromClass "/Game/SKYE/Blueprints/Multiplayer/MRTS_Player.MRTS_Player_C" (CallFunction|FindTeamPlayerStart (Utilities|String|StringToName (Utilities|String|EnumtoString team))) "Undefined" "MultiplyWithRoot" 0 0))
  (Pawn|Possess PlayerController _returnvalue_2)
  ;[1 1 1] initialise all units for the new player (needs to be done cos of how networking works)
  (bind _outactors (Actor|GetAllActorsOfClass "/Game/RORY/Multiplayer/Units/FriendlyUnits/FriendlyBPs/MBP_BaseUnit.MBP_BaseUnit_C"))
  (for _array_element _outactors
    (Default|SRInit _array_element)))

(fn SpawnKing
  (params (team :type Team%20Enum :default "NewEnumerator0"))
  (bind _returnvalue (Utilities|String|EnumtoString team))
  (bind _returnvalue_2 (Utilities|String|StringToName _returnvalue))
  (bind _startpos (CallFunction|FindTeamPlayerStart _returnvalue_2))
  ;[1 1 1] Spawns the king for each player
  ;;[1 1 1] rotate the king to face forwards depending on which team
  (switch Utilities|FlowControl|Switch|SwitchonTeam team
    (:NewEnumerator0
      (LocalVariables|Setrotation 9e+01)
      (bind _returnvalue_3 (Game|SpawnActorfromClass "/Game/RORY/Multiplayer/Units/FriendlyUnits/FriendlyBPs/MBP_FriendlyKing.MBP_FriendlyKing_C" (Math|Transform|MakeTransform (.location _startpos) (Math|Rotator|MakeRotator 0.0 0.0 (LocalVariables|Getrotation)) "1.000000,1.000000,1.000000") "Undefined" "MultiplyWithRoot" 0 0))
      ;;[1 1 1] set the team of the king
      (Variables|/Game/RORY/Multiplayer/Units/FriendlyUnits/FriendlyBPs/MBP_BaseUnit.MBP_BaseUnit_C|Setteam _returnvalue_3 "NewEnumerator0")
      (LocalVariables|SettheKing _returnvalue_3))
    (:NewEnumerator1
      (LocalVariables|Setrotation -9e+01)
      (bind _returnvalue_4 (Game|SpawnActorfromClass "/Game/RORY/Multiplayer/Units/FriendlyUnits/FriendlyBPs/MBP_FriendlyKing.MBP_FriendlyKing_C" (Math|Transform|MakeTransform (.location _startpos) (Math|Rotator|MakeRotator 0.0 0.0 (LocalVariables|Getrotation)) "1.000000,1.000000,1.000000") "Undefined" "MultiplyWithRoot" 0 0))
      (Variables|/Game/RORY/Multiplayer/Units/FriendlyUnits/FriendlyBPs/MBP_BaseUnit.MBP_BaseUnit_C|Setteam _returnvalue_4 "NewEnumerator1")
      (LocalVariables|SettheKing _returnvalue_4)))
  (return (LocalVariables|GettheKing)))

(fn SpawnUnit
  (params (PlayerState :type PS%20Multiplayer%20Object%20Reference) (UnitType :type Actor%20Class%20Reference) (location :type Vector) (team :type Team%20Enum :default "NewEnumerator0"))
  ;[1 1 1] spawn a new unit in the game
  (LocalVariables|Setloc location)
  (if (== UnitType "/Game/RORY/Multiplayer/Units/FriendlyUnits/FriendlyBPs/MBP_FriendlyRook.MBP_FriendlyRook_C")
    (LocalVariables|Setloc (+ (LocalVariables|Getloc) "0.000000,0.000000,1000.000000")))
  (switch Utilities|FlowControl|Switch|SwitchonTeam team
    (:NewEnumerator0
      (bind _returnvalue (Game|SpawnActorfromClass UnitType (Math|Transform|MakeTransform (LocalVariables|Getloc) "0.000000,90.000000,0.000000" "1.000000,1.000000,1.000000") "AdjustIfPossibleButAlwaysSpawn" "MultiplyWithRoot" 0 0))
      (bind _asmbp_base_unit (Utilities|Casting|CastToMBP_BaseUnit _returnvalue))
      (Variables|/Game/RORY/Multiplayer/Units/FriendlyUnits/FriendlyBPs/MBP_BaseUnit.MBP_BaseUnit_C|Setteam _asmbp_base_unit team)
      (return _asmbp_base_unit))
    (:NewEnumerator1
      (bind _returnvalue_2 (Game|SpawnActorfromClass UnitType (Math|Transform|MakeTransform (LocalVariables|Getloc) "0.000000,-90.000000,0.000000" "1.000000,1.000000,1.000000") "AdjustIfPossibleButAlwaysSpawn" "MultiplyWithRoot" 0 0))
      (bind _asmbp_base_unit_2 (Utilities|Casting|CastToMBP_BaseUnit _returnvalue_2))
      (Variables|/Game/RORY/Multiplayer/Units/FriendlyUnits/FriendlyBPs/MBP_BaseUnit.MBP_BaseUnit_C|Setteam _asmbp_base_unit_2 team)
      (return _asmbp_base_unit_2))))

(fn Endgame
  ;[1 1 1] end the game
  (if (not (LocalVariables|Gethasended))
    (LocalVariables|Sethasended true)
    (CallFunction|Stoptime) ; pause time for all players
    (bind _asgs_multiplayer (Utilities|Casting|CastToGS_Multiplayer (Game|GetGameState)))
    ;;[1 1 1] for each player, spawn the end game screen
    (for _array_element (Variables|Default|GetPlayers)
      (Default|End _array_element (Variables|/Game/SKYE/Blueprints/Multiplayer/Networking/Blueprints/GS_Multiplayer.GS_Multiplayer_C|GetLoser _asgs_multiplayer)))))

(fn BeginGame
  ;[1 1 1] Start the game
  (Utilities|FlowControl|Sequence
    (:then_0
      (CallFunction|ActivateAi))
    (:then_1
      (for _array_element (Variables|Default|GetPlayers)
        (bind _asps_multiplayer (Utilities|Casting|CastToPS_Multiplayer (Variables|/Script/Engine.Controller|GetPlayerState _array_element)))
        (Variables|/Game/SKYE/Blueprints/Multiplayer/Networking/Blueprints/PS_Multiplayer.PS_Multiplayer_C|SetcanControlUnits _asps_multiplayer true)
        (Variables|/Game/SKYE/Blueprints/Multiplayer/Networking/Blueprints/PS_Multiplayer.PS_Multiplayer_C|SetisPrepStage _asps_multiplayer false)))))

(fn ActivateAi
  ;[1 1 1] initialise the ai for the units (run the behaviour trees)
  (bind _outactors (Actor|GetAllActorsOfClass "/Game/RORY/Multiplayer/Units/FriendlyUnits/FriendlyBPs/MBP_BaseUnitController.MBP_BaseUnitController_C"))
  (for _array_element _outactors
    (Default|InitialiseAI _array_element)))

(fn DrawGame
  (if (not (LocalVariables|Getended))
    (LocalVariables|Setended true)
    (CallFunction|Stoptime) ; pause time for all players
    (for _array_element (Variables|Default|GetPlayers)
      (Default|Draw _array_element))))