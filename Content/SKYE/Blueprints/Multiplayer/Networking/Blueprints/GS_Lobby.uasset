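; Lobby game state that relays multiplayer lobby events for loading into the game and for players joining or leaving.
; SR_ events forward to MC_ events, which call each machine's local PC_Lobby to show the loading screen or add and remove player cards.
; Starting the game raises the loading screen first, waits briefly, then hands off to GM_Lobby to perform the load.
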(event Custom|SR_AddLobbyCard
  ;[1 1 1] create the card on the lobby screen to show that player has joined
  (CallFunction|MCAddLobbyCard))

(event Custom|SR_LoadGame
  ;[1 1 1] Load into the game
  (CallFunction|MCLoadingScreen)
  (Utilities|FlowControl|Delay 0.2)
  (bind _asgm_lobby (Utilities|Casting|CastToGM_Lobby (Game|GetGameMode)))
  (Default|SRLoadGame _asgm_lobby))

(event Custom|MC_AddLobbyCard
  ;[1 1 1] create the card on the lobby screen to show that player has joined
  (bind _aspc_lobby (Utilities|Casting|CastToPC_Lobby (Game|GetPlayerController 0)))
  (Default|AddLobbyCard _aspc_lobby))

(event Custom|MC_LoadingScreen
  ;[1 1 1] create loading screen on all clients
  (bind _aspc_lobby (Utilities|Casting|CastToPC_Lobby (Game|GetPlayerController 0)))
  (Default|LoadingScreen _aspc_lobby))

(event Custom|SR_removeCard
  ;[1 1 1] when player leaves, remove the player card from lobby screen
  (CallFunction|MCREmoveCard))

(event Custom|MC_REmoveCard
  ;[1 1 1] when player leaves, remove the player card from lobby screen
  (bind _aspc_lobby (Utilities|Casting|CastToPC_Lobby (Game|GetPlayerController 0)))
  (Default|RemoveLobbyCard _aspc_lobby))

(fn ConstructionScript)