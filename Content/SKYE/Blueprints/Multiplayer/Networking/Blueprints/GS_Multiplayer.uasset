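; Multiplayer game state that times the prep stage and match, telling GM_Multiplayer to begin the game or declare a draw.
; It also relays gameplay effects through SR_/MC_ event pairs: refund lockout, ragdolls, explosion effects, king status buffs, mesh reattachment and position fixes.
; Ragdoll and refund multicasts act through each machine's first MRTS_Controller, with authority checks choosing direct multicast or an SR_Call relay for ragdolls.
; King HP and prep-state OnRep functions are empty.
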(event Custom|SR_ExplodeRagdoll
  (params (mesh :type Skeletal%20Mesh%20Component%20Object%20Reference) (location :type Vector))
  ;[1 1 1] explosion ragdolling
  (bind _asmrts_controller (Utilities|Casting|CastToMRTS_Controller (Game|GetPlayerController 0)))
  (if (Ability|HasAuthority _asmrts_controller)
    (CallFunction|MCExplosionRagdoll location mesh)
    (else
      (CallFunction|SRCallExplodeRagdoll location mesh))))

(event Custom|SR_Unragdoll
  (params (mesh :type Skeletal%20Mesh%20Component%20Object%20Reference) (cap :type Capsule%20Component%20Object%20Reference))
  ;[1 1 1] unragdoll for units
  (Networking|SwitchHasAuthority
    (:Authority
      (CallFunction|MCUnragdoll mesh cap))
    (:Remote
      (CallFunction|SRCallUnragdoll mesh cap))))

(event Custom|SR_CallRagdoll
  (params (enemy :type Actor%20Object%20Reference) (unit :type Actor%20Object%20Reference) (mesh :type Skeletal%20Mesh%20Component%20Object%20Reference))
  ;[1 1 1] ragdolling for pawn
  (CallFunction|MCRagdoll enemy unit mesh))

(event Custom|SR_CallBuff
  (params (king :type MBP%20Friendly%20King%20Object%20Reference) (status :type KingStatus%20Enum :default "NewEnumerator0"))
  (CallFunction|MCCallBuff status king))

(event Custom|MC_CallBuff
  (params (status :type KingStatus%20Enum :default "NewEnumerator0") (king :type MBP%20Friendly%20King%20Object%20Reference))
  (Default|SwitchStatusEffect king status))

(event Custom|SR_CheckBeneathFloorWorld
  (params (Unit :type Skeletal%20Mesh%20Component%20Object%20Reference) (Location :type Vector))
  (CallFunction|MCCheckBeneathFloorWorld Unit Location))

(event Custom|SR_CallExplodeRagdoll
  (params (location :type Vector) (mesh :type Skeletal%20Mesh%20Component%20Object%20Reference))
  ;[1 1 1] explosion ragdolling
  (CallFunction|MCExplosionRagdoll location mesh))

(event Custom|MC_CheckBeneathFloorWorld
  (params (Unit :type Skeletal%20Mesh%20Component%20Object%20Reference) (Location :type Vector))
  (Transformation|SetWorldLocation Unit Location false true))

(event Custom|MC_ExplosionRagdoll
  (params (location :type Vector) (Mesh :type Skeletal%20Mesh%20Component%20Object%20Reference))
  ;[1 1 1] explosion ragdolling
  (bind _asmrts_controller (Utilities|Casting|CastToMRTS_Controller (Game|GetPlayerController 0)))
  (Default|RocketRagdoll _asmrts_controller location Mesh))

(event Custom|SR_CheckBeneathFloorActor
  (params (Unit :type MBP%20Base%20Unit%20Object%20Reference) (Location :type Vector))
  (CallFunction|MCCheckBeneathFloorActor Unit Location))

(event Custom|MC_CheckBeneathFloorActor
  (params (Unit :type MBP%20Base%20Unit%20Object%20Reference) (Location :type Vector))
  (Transformation|SetActorLocation Unit Location false false))

(event Custom|SR_Reattach
  (params (capsule :type Capsule%20Component%20Object%20Reference) (mesh :type Skeletal%20Mesh%20Component%20Object%20Reference))
  (CallFunction|MCReattach mesh capsule))

(event Custom|SR_Ragdoll
  (params (mesh :type Skeletal%20Mesh%20Component%20Object%20Reference) (enemy :type Actor%20Object%20Reference) (unit :type Actor%20Object%20Reference))
  ;[1 1 1] ragdolling for pawn
  (bind _asmrts_controller (Utilities|Casting|CastToMRTS_Controller (Game|GetPlayerController 0)))
  (if (Ability|HasAuthority _asmrts_controller)
    (CallFunction|MCRagdoll enemy unit mesh)
    (else
      (CallFunction|SRCallRagdoll enemy unit mesh))))

(event Custom|MC_Reattach
  (params (mesh :type Skeletal%20Mesh%20Component%20Object%20Reference) (capsule :type Capsule%20Component%20Object%20Reference))
  (Transformation|AttachComponentToComponent mesh capsule "None" "KeepRelative" "KeepRelative" "KeepWorld" true)
  (Transformation|SetRelativeLocationAndRotation mesh "0.000000,0.000000,-90.000000" "0.0,270.0,0.0" false false))

(event Custom|MC_Ragdoll
  (params (Enemy :type Actor%20Object%20Reference) (Unit :type Actor%20Object%20Reference) (Mesh :type Skeletal%20Mesh%20Component%20Object%20Reference))
  ;[1 1 1] ragdolling for pawn
  (bind _asmrts_controller (Utilities|Casting|CastToMRTS_Controller (Game|GetPlayerController 0)))
  (Default|RagdollEvent _asmrts_controller Mesh Enemy Unit))

(event Custom|MC_SpawnBoom
  (params (location :type Vector) (particle :type Niagara%20System%20Object%20Reference) (sfx :type Sound%20Base%20Object%20Reference) (dilation :type Float%20%28double-precision%29))
  (bind _returnvalue (Niagara|SpawnSystematLocation particle location "0, 0, 0" "5.000000,5.000000,5.000000"))
  (Utilities|IsValid _returnvalue
    (:Is%20Valid
      (Class|NiagaraComponent|SetCustomTimeDilation _returnvalue dilation)
      (Audio|SpawnSoundatLocation sfx location "0, 0, 0" 1.0 1.0 0.0 0 0)
      (Development|PrintString "Hello"))
    (:Is%20Not%20Valid
      (Development|PrintString "failed to spawn particle"))))

(event Custom|SR_SpawnBoom
  (params (location :type Vector) (particle :type Niagara%20System%20Object%20Reference) (sfx :type Sound%20Base%20Object%20Reference) (dilation :type Float%20%28double-precision%29))
  (CallFunction|MCSpawnBoom location particle sfx dilation))

(event Custom|SR_DisableAllRefunds
  ;[1 1 1] disable refund button for all players at end of preparation stage
  (CallFunction|MCDisableallrefunds))

(event Custom|SR_CallUnragdoll
  (params (Mesh :type Skeletal%20Mesh%20Component%20Object%20Reference) (col :type Capsule%20Component%20Object%20Reference))
  ;[1 1 1] unragdoll for units
  (CallFunction|MCUnragdoll Mesh col))

(event Custom|MC_Unragdoll
  (params (mesh :type Skeletal%20Mesh%20Component%20Object%20Reference) (Cap :type Capsule%20Component%20Object%20Reference))
  ;[1 1 1] unragdoll for units
  (bind _asmrts_controller (Utilities|Casting|CastToMRTS_Controller (Game|GetPlayerController 0)))
  (Default|UnRagdollEvent _asmrts_controller mesh Cap))

(event Custom|MC_Disableallrefunds
  ;[1 1 1] disable refund button for all players at end of preparation stage
  (bind _asmrts_controller (Utilities|Casting|CastToMRTS_Controller (Game|GetPlayerController 0)))
  (Default|DisableRefundBtn _asmrts_controller))

(event EventTick
  (params (DeltaSeconds :type Float%20%28single-precision%29))
  (if (Variables|Default|Getprepstage)
    ;[1 1 1] Countdown for prep stage, begin game once prep stage is over
    (bind _output_get (Variables|Default|SetPrepCountdown (- (Variables|Default|GetPrepCountdown) DeltaSeconds)))
    (if (<= _output_get 0.0)
      (Variables|Default|Setprepstage false)
      (bind _asgm_multiplayer (Utilities|Casting|CastToGM_Multiplayer (Game|GetGameMode)))
      (Default|BeginGame _asgm_multiplayer)
      (CallFunction|SRDisableAllRefunds))
    (else
      ;[1 1 1] countdown until game is over
      (CallFunction|Countdown DeltaSeconds))))

(fn ConstructionScript)

(fn OnRepKing1hp)

(fn OnRepKing2hp)

(fn OnRepPrepCountdown)

(fn OnRepPrepstage)

(fn Countdown
  (params (tick :type Float%20%28double-precision%29))
  ;[1 1 1] Counts down to zero and ends game when it hits 0
  (bind _output_get (Variables|Default|Settimeremaining (- (Variables|Default|Gettimeremaining) tick)))
  (if (and (<= _output_get 0.0) (not (Variables|Default|GetDrawState)))
    (Variables|Default|SetDrawState true)
    (bind _asgm_multiplayer (Utilities|Casting|CastToGM_Multiplayer (Game|GetGameMode)))
    (Default|DrawGame _asgm_multiplayer)))