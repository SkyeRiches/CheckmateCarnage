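; Player controller for the multiplayer lobby that creates the lobby UI, shows the cursor and adds a start button for player 1, the host.
; Events add and remove player cards on that UI after a one-tick delay, with card removal also forwarded to GS_Lobby.
; It also shows a loading screen, stores the chosen team in the game instance, and destroys the session to return to the menu when kicked.
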(event Custom|RemoveLobbyCard
  ;[1 1 1] remove player card from lobby screen
  (Utilities|FlowControl|DelayUntilNextTick)
  (Default|RemoveCard (Variables|Default|Gethud)))

(event Custom|LoadingScreen
  ;[1 1 1] Spawn Loading screen
  (bind _returnvalue (UserInterface|CreateWidget "/Game/SKYE/Blueprints/Multiplayer/Networking/widgets/WB_Loading.WB_Loading_C" (Game|GetPlayerController 0)))
  (UserInterface|Viewport|AddtoViewport _returnvalue 0))

(event Custom|OC_KickedFromLobby
  ;[1 1 1] return to menu if kicked from lobby (only happens if the host quits)
  (|DestroySession self
    (:OnSuccess
      (Game|OpenLevel(byObjectReference) "/Game/Menu.Menu"))))

(event Custom|AddLobbyCard
  ;[1 1 1] add the player card to the lobby
  (Utilities|FlowControl|DelayUntilNextTick)
  (Default|AddPlayerCard (Variables|Default|Gethud)))

(event Custom|SetTeam
  (params (NewParam :type Team%20Enum :default "NewEnumerator0"))
  (bind _output_get (Variables|Default|Setteam NewParam))
  (bind _asgi_checkmate_carnage_steam (Utilities|Casting|CastToGI_CheckmateCarnageSteam (Game|GetGameInstance)))
  (bind _output_get_2 (Variables|/Game/SKYE/Blueprints/Multiplayer/Networking/Blueprints/GI_CheckmateCarnageSteam.GI_CheckmateCarnageSteam_C|SetTeam _asgi_checkmate_carnage_steam _output_get))
  (Development|PrintString (Utilities|String|EnumtoString _output_get_2)))

(event Custom|SR_RemoveCard
  ;[1 1 1] remove player card from lobby screen
  (bind _asgs_lobby (Utilities|Casting|CastToGS_Lobby (Game|GetGameState)))
  (Default|SRRemoveCard _asgs_lobby))

(event EventBeginPlay
  ;[1 1 1] spawn the hud for the lobby screen
  (bind _returnvalue (UserInterface|CreateWidget "/Game/SKYE/Blueprints/Multiplayer/Networking/widgets/WB_LobbyUI.WB_LobbyUI_C" (Game|GetPlayerController 0)))
  (UserInterface|Viewport|AddtoViewport _returnvalue 0)
  (Variables|Default|Sethud _returnvalue)
  (Variables|Default|SetbShowMouseCursor true)
  (Utilities|FlowControl|DelayUntilNextTick)
  (switch int (Variables|Default|Getplayernum)
    (:1
      (Default|AddStartButton (Variables|Default|Gethud)) ; is player 1 add a start button (only host can start game)
    )))

(fn ConstructionScript)