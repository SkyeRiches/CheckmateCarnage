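; GM_Lobby is the multiplayer lobby game mode that registers joining players and starts the match.
; On PostLogin it adds each PC_Lobby to its player list, gives the first and second players different teams, and assigns player numbers.
; When player two joins, it waits briefly, then has GS_Lobby add a lobby card showing the connection.
; SR_LoadGame sends everyone to the map named by MapName via a servertravel console command.
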(event Custom|SR_LoadGame
  ;[1 1 1] travel to the multiplayer level
  (Development|ExecuteConsoleCommand (Utilities|String|Append "servertravel /Game/" (Variables|Default|GetMapName)) (Game|GetPlayerController 0)))

(event EventPostLogin
  (params (NewPlayer :type Player%20Controller%20Object%20Reference))
  (bind _players (Variables|Default|GetPlayers))
  ;[1 1 1] when a new player joins, add them to list of player and increase num of players
  (bind _aspc_lobby (Utilities|Casting|CastToPC_Lobby NewPlayer))
  (bind _returnvalue (Utilities|Array|AddUnique _players _aspc_lobby))
  (switch int (Utilities|Array|Length _players)
    (:1
      (Default|SetTeam _aspc_lobby "NewEnumerator0"))
    (:2
      (Default|SetTeam _aspc_lobby "NewEnumerator1")))
  (bind _output_get (Variables|/Game/SKYE/Blueprints/Multiplayer/Networking/Blueprints/PC_Lobby.PC_Lobby_C|Setplayernum _aspc_lobby (+ _returnvalue 1)))
  (switch int _output_get ; if player 2 joined
    (:2
      ;[1 1 1] create the player two card on the lobby to show that player 2 has connected
      (Utilities|FlowControl|Delay 0.2)
      (bind _asgs_lobby (Utilities|Casting|CastToGS_Lobby (Game|GetGameState)))
      (Default|SRAddLobbyCard _asgs_lobby))))

(fn ConstructionScript)