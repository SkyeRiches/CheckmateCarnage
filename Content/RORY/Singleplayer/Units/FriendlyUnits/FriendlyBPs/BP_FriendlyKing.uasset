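; Friendly king unit that supports units around it with a switchable heal, speed or damage aura.
; BuffRadius overlaps maintain the units-in-range list, removing the speed buff on exit.
; Tick heals listed units in Heal mode, while SwitchStatusEffect applies speed or damage buffs once, swapping out the other.
; At zero HP it reports the king's death to BP_EndgameManager, stops its AI and destroys controller and pawn.
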(event OnComponentBeginOverlap(BuffRadius)
  (params (OverlappedComponent :type Primitive%20Component%20Object%20Reference) (OtherActor :type Actor%20Object%20Reference) (OtherComp :type Primitive%20Component%20Object%20Reference) (OtherBodyIndex :type Integer) (bFromSweep :type Boolean) (SweepResult :type Hit%20Result%20Structure%20%28by%20ref%29))
  ;[1 1 1] Add allied units in range to list - skye
  (bind _asbp_base_unit (Utilities|Casting|CastToBP_BaseUnit OtherActor))
  (Utilities|Array|AddUnique (Variables|Default|GetUnitsInRange) _asbp_base_unit))

(event OnComponentEndOverlap(BuffRadius)
  (params (OverlappedComponent :type Primitive%20Component%20Object%20Reference) (OtherActor :type Actor%20Object%20Reference) (OtherComp :type Primitive%20Component%20Object%20Reference) (OtherBodyIndex :type Integer))
  ;[1 1 1] Remove any allied units not in range - skye
  (bind _asbp_base_unit (Utilities|Casting|CastToBP_BaseUnit OtherActor))
  (Default|RemoveSpeedBuff _asbp_base_unit)
  (Utilities|Array|RemoveItem (Variables|Default|GetUnitsInRange) _asbp_base_unit))

(event EventTick
  (params (DeltaSeconds :type Float%20%28single-precision%29))
  (bind _self self)
  (bind _returnvalue (AI|GetAIController _self))
  (Variables|Default|SetDeltaTime DeltaSeconds)
  (if (<= (Variables|Default|GetHP) 0.0) ; if should die
    ;[1 1 1] Tell the end game the king has died, then stop the ai for the king and destroy itself - skye
    (bind _returnvalue_2 (Actor|GetActorOfClass "/Game/SKYE/Blueprints/Singleplayer/Endgame/BP_EndgameManager.BP_EndgameManager_C"))
    (Default|KingDeath _returnvalue_2 false)
    (AI|Logic|StopLogic (Variables|/Script/AIModule.AIController|GetBrainComponent _returnvalue) "")
    (Actor|DestroyActor _returnvalue)
    (Actor|DestroyActor)
    (else
      (|CallParentFunction (Variables|Default|GetDeltaTime))
      ;[1 1 1] Heal all allies in range - skye
      (if (Utilities|Enum|Equal(Enum) (Variables|Default|GetStatusEffect) "NewEnumerator0")
        (for _array_element (Variables|Default|GetUnitsInRange)
          (Default|Heal _array_element (* (Variables|Default|GetKingHealPower) (Variables|Default|GetDeltaTime))))))))

(fn ConstructionScript
  (|CallParentFunction))

(fn SwitchStatusEffect
  (params (Status :type KingStatus%20Enum :default "NewEnumerator0"))
  ;[1 1 1] change which status effec the king has - skye
  (bind _output_get (Variables|Default|SetStatusEffect Status))
  (switch Utilities|FlowControl|Switch|SwitchonKingStatus _output_get
    (:NewEnumerator1
      (for _array_element (Variables|Default|GetUnitsInRange)
        (Default|SpeedBuff _array_element 2.0)
        (bind _asbp_base_unit_controller (Utilities|Casting|CastToBP_BaseUnitController (AI|GetAIController _array_element)))
        (Default|RemoveDamageBuff _asbp_base_unit_controller)))
    (:NewEnumerator2
      (for _array_element_2 (Variables|Default|GetUnitsInRange)
        (Default|RemoveSpeedBuff _array_element_2)
        (bind _asbp_base_unit_controller_2 (Utilities|Casting|CastToBP_BaseUnitController (AI|GetAIController _array_element_2)))
        (Default|BuffDamage _asbp_base_unit_controller_2 2.0)))))