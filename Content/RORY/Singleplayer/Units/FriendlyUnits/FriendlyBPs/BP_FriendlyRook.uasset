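; BP_FriendlyRook is a friendly Rook unit for singleplayer that acquires enemy targets for its AI.
; It uses large rectangular colliders for targeting in place of AI senses.
; When a BP_BaseEnemy overlaps it, it writes that enemy to the NearestEnemy key on the BP_FriendlyRookController blackboard, only if no valid target is set.
; The target is therefore the first enemy to overlap, with no distance comparison.
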(event EventBeginPlay
  ;[1 1 1] Instead of using senses, the rook uses large rectangular colliders to set its target
  (|CallParentFunction) ; This node is disabled and will not be called.\nDrag off pins to build functionality.
)

(event Collision|EventActorBeginOverlap
  (params (OtherActor :type Actor%20Object%20Reference))
  (bind _returnvalue (Utilities|Name|MakeLiteralName "NearestEnemy"))
  ;[1 1 1] Instead of using senses, the rook uses large rectangular colliders to set its target
  (bind _asbp_base_enemy (Utilities|Casting|CastToBP_BaseEnemy OtherActor))
  (bind _asbp_friendly_rook_controller (Utilities|Casting|CastToBP_FriendlyRookController (Pawn|GetController (Variables|Default|GetTarget))))
  (if (Utilities|IsValid (AI|GetBlackboard _asbp_friendly_rook_controller))
    (Utilities|IsValid (AI|Components|Blackboard|GetValueasObject (AI|GetBlackboard _asbp_friendly_rook_controller) _returnvalue)
      (:Is%20Not%20Valid
        (AI|Components|Blackboard|SetValueasObject (AI|GetBlackboard _asbp_friendly_rook_controller) _returnvalue _asbp_base_enemy)))))

(event EventTick
  (params (DeltaSeconds :type Float%20%28single-precision%29))
  (|CallParentFunction DeltaSeconds) ; This node is disabled and will not be called.\nDrag off pins to build functionality.
)

(fn ConstructionScript
  (|CallParentFunction))