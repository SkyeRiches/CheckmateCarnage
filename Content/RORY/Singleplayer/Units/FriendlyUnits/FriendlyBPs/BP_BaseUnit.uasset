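; Base friendly AI unit character with health, damage and healing, speed buffs, and selection visuals.
; A dynamic decal material recolours the selection ring, and custom depth stencil values drive the highlight shader.
; Tick emits noise for detection, turns the health bar toward the camera, and destroys the unit and controller at zero HP.
; While ragdolled, the capsule follows the pelvis until a timer allows recovery, which reattaches the mesh.
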(event EventBeginPlay
  ;[1 1 1] Initialise the units properties - skye
  (CallFunction|RingDefaultColor)
  (Variables|Default|SetHP (Variables|Default|GetMaxHealth))
  (Class|PrimitiveComponent|WakeAllRigidBodies (Variables|Character|GetMesh)))

(event EventTick
  (params (DeltaSeconds :type Float%20%28single-precision%29))
  (bind _self self)
  (bind _healthbar (Variables|Default|GetHealthBar))
  (bind _returnvalue (AI|GetAIController _self))
  ;[1 1 1] Make noise so other units can detect it
  (Class|Actor|MakeNoise 1.0 0 "0, 0, 0" 0.0 "None")
  ;[1 1 1] Update health bar and make it point towards camera
  (bind _ashealth_bar (Utilities|Casting|CastToHealthBar (UserInterface|GetWidget (Variables|Default|GetHealthBar))))
  (bind _output_get (Variables|Default|SetHPPercentage (/ (Variables|Default|GetHP) (Variables|Default|GetMaxHealth))))
  (Progress|SetPercent (Variables|/Game/RORY/HealthBar.HealthBar_C|GetHealthBar _ashealth_bar) _output_get)
  (Transformation|SetWorldRotation _healthbar (Math|Rotator|FindLookatRotation (Transformation|GetWorldLocation _healthbar) (Transformation|GetWorldLocation (Variables|/Script/Engine.PlayerCameraManager|GetTransformComponent (Game|GetPlayerCameraManager 0)))) false false)
  ;[1 1 1] Unragdoll if ragdolltime has reached 0
  (if (Variables|Default|GetIsRagdoll)
    (Transformation|SetWorldLocation (Variables|Collision|GetCapsuleComponent) (Transformation|GetSocketLocation (Variables|Character|GetMesh) "Pelvis") false false)
    (Variables|Default|SetUnragdollTime (- (Variables|Default|GetUnragdollTime) (Utilities|Time|GetWorldDeltaSeconds)))
    (if (< (Variables|Default|GetUnragdollTime) 1.5)
      (if (Variables|Default|GetCan%20Start%20Getting%20Up)
        (CallFunction|Unragdoll)
        ;[1 1 1] Tell the blackboard if the unit is ragdolled
        (if (< (Variables|Default|GetUnragdollTime) 0.0)
          (AI|Components|Blackboard|SetValueasBool (AI|GetBlackboard 0) (Utilities|Name|MakeLiteralName "IsRagdoll") false)))))
  ;[1 1 1] Death
  (if (<= (Variables|Default|GetHP) 0.0)
    (AI|Logic|StopLogic (Variables|/Script/AIModule.AIController|GetBrainComponent _returnvalue) "")
    (Actor|DestroyActor _returnvalue)
    (Actor|DestroyActor)))

(fn ConstructionScript
  (bind _returnvalue (Rendering|Material|CreateDynamicMaterialInstance (Variables|Default|GetDecal) :!class /Script/Engine.DecalComponent))
  (Variables|Default|SetMaterial _returnvalue))

(fn TakeDamage
  (params (DMG :type Float%20%28double-precision%29))
  ;[1 1 1] reduce hp by amount - skye
  (Variables|Default|SetHP (- (Variables|Default|GetHP) DMG)))

(fn RingSelectColor
  ;[1 1 1] Set the ring decal to be white - skye
  (Rendering|Material|SetVectorParameterValue (Variables|Default|GetMaterial) "RingColor" (Math|Conversions|ToLinearColor(Color) (Variables|Default|GetSelectRingColor)) :!class /Script/Engine.MaterialInstanceDynamic)
  (Rendering|Material|SetScalarParameterValue (Variables|Default|GetMaterial) "EmissionStrength" (Variables|Default|GetSelectEmissionStrength) :!class /Script/Engine.MaterialInstanceDynamic))

(fn RingDefaultColor
  ;[1 1 1] Set the decal ring to be blue - skye
  (Rendering|Material|SetVectorParameterValue (Variables|Default|GetMaterial) "RingColor" (Math|Conversions|ToLinearColor(Color) (Variables|Default|GetDefaultRingColor)) :!class /Script/Engine.MaterialInstanceDynamic)
  (Rendering|Material|SetScalarParameterValue (Variables|Default|GetMaterial) "EmissionStrength" (Variables|Default|GetDefaultEmissionStrength) :!class /Script/Engine.MaterialInstanceDynamic))

(fn HighlightUnit
  (params (StencilLayer :type Integer))
  (bind _mesh (Variables|Character|GetMesh))
  ;[1 1 1] Set the unit to be on the stencil layer to highlight them using the highlight shader - skye
  (Rendering|SetRenderCustomDepth _mesh true)
  (Rendering|SetCustomDepthStencilValue _mesh StencilLayer))

(fn UnHighlightUnit
  ;[1 1 1] set it to not be on custom render depth so that it doesnt get highlighted - skye
  (Rendering|SetRenderCustomDepth (Variables|Character|GetMesh) false))

(fn Unragdoll
  (bind _mesh (Variables|Character|GetMesh))
  (bind _mesh_2 (Variables|Character|GetMesh))
  (bind _returnvalue (Transformation|GetSocketLocation _mesh_2 "pelvis"))
  (bind (_x _y _z) (Math|Vector|BreakVector _returnvalue))
  ;[1 1 1] Attatch the capsule component to the pelvis
  (Transformation|SetWorldLocation (Variables|Collision|GetCapsuleComponent) (Math|Vector|MakeVector _x _y (+ _z 1e+02)) false false)
  ;[1 1 1] Disable ragdoll variable and set physics to not be simulated
  (Physics|SetSimulatePhysics (Variables|Character|GetMesh) false)
  (Variables|Default|SetIsRagdoll false)
  (bind _returnvalue_2 (Collision|LineTraceByChannel _returnvalue (+ _returnvalue (* (Math|Vector|GetRightVector (Transformation|GetSocketRotation _mesh_2 "Pelvis")) 5e+01)) "TraceTypeQuery1" false 0 "None"))
  (if _returnvalue_2 ; play animation depending on outcome
    _
    (else
      _))
  (Physics|SetSimulatePhysics _mesh false)
  ;[1 1 1] Attatch mesh to capsule
  (Transformation|AttachComponentToComponent _mesh (Variables|Collision|GetCapsuleComponent) "None" "KeepRelative" "KeepRelative" "KeepWorld" true)
  (Transformation|SetRelativeLocationAndRotation (Variables|Character|GetMesh) "0.000000,0.000000,-95.000000" "0.0,270.0,0.0" false false)
  (Input|EnableInput 0))

(fn Heal
  (params (HealAmount :type Float%20%28double-precision%29))
  ;[1 1 1] increase hp by specified amount - skye
  (Variables|Default|SetHP (+ (Variables|Default|GetHP) HealAmount)))

(fn SpeedBuff
  (params (Modifier :type Float%20%28double-precision%29))
  ;[1 1 1] increase move speed - skye
  (Variables|/Script/Engine.CharacterMovementComponent|SetMaxWalkSpeed (Variables|Character|GetCharacterMovement) (* (Variables|Default|GetBaseMoveSpeed) Modifier)))

(fn RemoveSpeedBuff
  ;[1 1 1] sets move speed back to normal - skye
  (Variables|/Script/Engine.CharacterMovementComponent|SetMaxWalkSpeed (Variables|Character|GetCharacterMovement) (Variables|Default|GetBaseMoveSpeed)))