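; AI controller for the friendly knight unit in singleplayer, built on a parent controller that defines an InitialiseAI step.
; Its InitialiseAI override calls the parent, runs a behavior tree, then sets the Moving and Attacking blackboard flags to false.
; BeginPlay, the construction script and a second InitialiseAI_0 graph only forward to the parent, and Tick is unused.
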(event EventBeginPlay
  (|CallParentFunction))

(event EventTick
  (params (DeltaSeconds :type Float%20%28single-precision%29)))

(fn ConstructionScript
  (|CallParentFunction))

(fn InitialiseAI0
  (|CallParentFunction))

(fn InitialiseAI
  (|CallParentFunction)
  (AI|RunBehaviorTree (Variables|Default|GetBehaviourTree))
  (AI|Components|Blackboard|SetValueasBool (Variables|Default|GetBlackboard) (Utilities|Name|MakeLiteralName "Moving") false)
  (AI|Components|Blackboard|SetValueasBool (Variables|Default|GetBlackboard) (Utilities|Name|MakeLiteralName "Attacking") false))