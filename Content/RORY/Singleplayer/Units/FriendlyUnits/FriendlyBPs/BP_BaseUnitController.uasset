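; Base AI controller for friendly units, running a behavior tree and feeding it targets through the Blackboard.
; Perception updates write enemies to NearestEnemy and other units to Ally, with no distance check, so later entries overwrite earlier ones.
; Tick counts down the Blackboard Cooldown, InitialiseAI starts the tree, and two functions apply or remove a multiplier on base damage.
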(event OnPerceptionUpdated(AIPerception)
  (params (UpdatedActors :type Array%20of%20Actor%20Object%20References))
  (bind _blackboard (Variables|Default|GetBlackboard))
  (if (Utilities|IsValid (AI|GetBlackboard 0))
    ;[1 1 1] set nearest enemy as first unit seen
    (for _array_element UpdatedActors
      (bind _asbp_base_enemy (Utilities|Casting|CastToBP_BaseEnemy _array_element)
        (:then
          (AI|Components|Blackboard|SetValueasObject _blackboard (Utilities|Name|MakeLiteralName "NearestEnemy") _asbp_base_enemy))
        (:CastFailed
          ;[1 1 1] If unit is on the same team set it as ally
          (bind _asbp_base_unit (Utilities|Casting|CastToBP_BaseUnit _array_element))
          (if (not (== _asbp_base_unit (Pawn|GetControlledPawn)))
            (AI|Components|Blackboard|SetValueasObject _blackboard (Utilities|Name|MakeLiteralName "Ally") _asbp_base_unit)))))))

(event EventTick
  (params (DeltaSeconds :type Float%20%28single-precision%29))
  (bind _returnvalue (Utilities|Name|MakeLiteralName "Cooldown"))
  (bind _blackboard (Variables|Default|GetBlackboard))
  ;[1 1 1] Lower cooldown each frame
  (if (Utilities|IsValid (AI|GetBlackboard 0))
    (AI|Components|Blackboard|SetValueasFloat _blackboard _returnvalue (- (Class|BlackboardComponent|GetValueasFloat _blackboard _returnvalue) DeltaSeconds))))

(fn ConstructionScript)

(fn InitialiseAI
  ;[1 1 1] Initialise the base ai - skye
  (AI|RunBehaviorTree (Variables|Default|GetBehaviourTree)))

(fn BuffDamage
  (params (Modifier :type Float%20%28double-precision%29))
  (Variables|Default|SetDamage (* (Variables|Default|GetBaseDamage) Modifier)))

(fn RemoveDamageBuff
  ;[1 1 1] returns damage back to normal  - skye
  (Variables|Default|SetDamage (Variables|Default|GetBaseDamage)))