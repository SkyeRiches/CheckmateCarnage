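; BP_EnemyKing is the singleplayer enemy king unit, which heals nearby units and reports its death to the endgame.
; BuffRadius overlaps maintain UnitsInRange, admitting only BP_BaseUnit actors without the "Enemy" tag, though comments call them allies.
; Tick heals that list by KingHealPower scaled by delta time.
; At zero HP, it notifies BP_EndgameManager, stops its AI logic and destroys both controller and itself.
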(event OnComponentBeginOverlap(BuffRadius)
  (params (OverlappedComponent :type Primitive%20Component%20Object%20Reference) (OtherActor :type Actor%20Object%20Reference) (OtherComp :type Primitive%20Component%20Object%20Reference) (OtherBodyIndex :type Integer) (bFromSweep :type Boolean) (SweepResult :type Hit%20Result%20Structure%20%28by%20ref%29))
  ;[1 1 1] Add allied units in range to list
  (bind _asbp_base_unit (Utilities|Casting|CastToBP_BaseUnit OtherActor))
  (if (not (Actor|ActorHasTag _asbp_base_unit "Enemy"))
    (Utilities|Array|AddUnique (Variables|Default|GetUnitsInRange) _asbp_base_unit)))

(event OnComponentEndOverlap(BuffRadius)
  (params (OverlappedComponent :type Primitive%20Component%20Object%20Reference) (OtherActor :type Actor%20Object%20Reference) (OtherComp :type Primitive%20Component%20Object%20Reference) (OtherBodyIndex :type Integer))
  ;[1 1 1] Remove any allied units not in range
  (bind _asbp_base_unit (Utilities|Casting|CastToBP_BaseUnit OtherActor))
  (if (not (Actor|ActorHasTag _asbp_base_unit "Enemy"))
    (Utilities|Array|RemoveItem (Variables|Default|GetUnitsInRange) _asbp_base_unit)))

(event EventBeginPlay
  (|CallParentFunction) ; This node is disabled and will not be called.\nDrag off pins to build functionality.
)

(event Collision|EventActorBeginOverlap
  (params (OtherActor :type Actor%20Object%20Reference)))

(event EventTick
  (params (DeltaSeconds :type Float%20%28single-precision%29))
  (bind _self self)
  (bind _returnvalue (AI|GetAIController _self))
  (if (<= (Variables|Default|GetHP) 0.0) ; if should die
    ;[1 1 1] Tell the end game the king has died, then stop the ai for the king and destroy itself - skye
    (bind _returnvalue_2 (Actor|GetActorOfClass "/Game/SKYE/Blueprints/Singleplayer/Endgame/BP_EndgameManager.BP_EndgameManager_C"))
    (Default|KingDeath _returnvalue_2 true)
    (AI|Logic|StopLogic (Variables|/Script/AIModule.AIController|GetBrainComponent _returnvalue) "")
    (Actor|DestroyActor _returnvalue)
    (Actor|DestroyActor)
    (else
      (|CallParentFunction DeltaSeconds)
      ;[1 1 1] Heal all allies in range - skye
      (for _array_element (Variables|Default|GetUnitsInRange)
        (bind _asbp_base_unit (Utilities|Casting|CastToBP_BaseUnit _array_element))
        (Default|Heal _asbp_base_unit (* (Variables|Default|GetKingHealPower) DeltaSeconds))))))

(fn ConstructionScript
  (|CallParentFunction))