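; Base AI controller for singleplayer enemy units, running a behavior tree and feeding its Blackboard.
; InitialiseAI starts the tree, clears the Moving and Attacking flags, and stores both enemy royals and the friendly king; the FriendlyQueen setter is unconnected.
; Perception updates write units without the Enemy tag to NearestEnemy, with no distance check.
; Tick counts down the Blackboard Cooldown.
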(event OnPerceptionUpdated(AIPerception)
  (params (UpdatedActors :type Array%20of%20Actor%20Object%20References))
  ;[1 1 1] if spotted a unit that isnt an ally, target that unit
  (if (Utilities|IsValid (AI|GetBlackboard 0))
    (for _array_element UpdatedActors
      (bind _asbp_base_unit (Utilities|Casting|CastToBP_BaseUnit _array_element))
      (if (not (Actor|ActorHasTag _asbp_base_unit "Enemy"))
        (AI|Components|Blackboard|SetValueasObject (AI|GetBlackboard 0) (Utilities|Name|MakeLiteralName "NearestEnemy") _asbp_base_unit)))))

(event EventTick
  (params (DeltaSeconds :type Float%20%28single-precision%29))
  (bind _returnvalue (Utilities|Name|MakeLiteralName "Cooldown"))
  (bind _blackboard (Variables|Default|GetBlackboard))
  (if (Utilities|IsValid (AI|GetBlackboard 0))
    (AI|Components|Blackboard|SetValueasFloat _blackboard _returnvalue (- (Class|BlackboardComponent|GetValueasFloat _blackboard _returnvalue) DeltaSeconds))))

(event EventBeginPlay)

(fn ConstructionScript)

(fn InitialiseAI
  ;[1 1 1] Initialise ai
  (AI|RunBehaviorTree (Variables|Default|GetBehaviourTree))
  (AI|Components|Blackboard|SetValueasBool (Variables|Default|GetBlackboard) (Utilities|Name|MakeLiteralName "Moving") false)
  (AI|Components|Blackboard|SetValueasBool (Variables|Default|GetBlackboard) (Utilities|Name|MakeLiteralName "Attacking") false)
  (bind _returnvalue (Actor|GetActorOfClass "/Game/RORY/Singleplayer/Units/EnemyUnits/Blueprints/BP_EnemyKing.BP_EnemyKing_C"))
  (AI|Components|Blackboard|SetValueasObject (Variables|Default|GetBlackboard) (Utilities|Name|MakeLiteralName "EnemyKing") _returnvalue)
  (bind _returnvalue_2 (Actor|GetActorOfClass "/Game/RORY/Singleplayer/Units/EnemyUnits/Blueprints/BP_EnemyQueen.BP_EnemyQueen_C"))
  (AI|Components|Blackboard|SetValueasObject (Variables|Default|GetBlackboard) (Utilities|Name|MakeLiteralName "EnemyQueen") _returnvalue_2)
  (bind _returnvalue_3 (Actor|GetActorOfClass "/Game/RORY/Singleplayer/Units/FriendlyUnits/FriendlyBPs/BP_FriendlyKing.BP_FriendlyKing_C"))
  (AI|Components|Blackboard|SetValueasObject (Variables|Default|GetBlackboard) (Utilities|Name|MakeLiteralName "FriendlyKing") _returnvalue_3))