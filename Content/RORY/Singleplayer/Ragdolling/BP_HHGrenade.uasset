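; BP_HHGrenade is a grenade projectile actor that flies in an arc and bursts on overlap, playing a splash sound and destroying itself.
; Initialize caches the starting location, then Tick integrates gravity into a tracked velocity and moves the actor manually without sweeping.
; A countdown grace period blocks detonation until it drops below zero, and Explode resets it before destroying the actor.
; The explosion applies no damage or physics force here.
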(event Collision|EventActorBeginOverlap
  (params (OtherActor :type Actor%20Object%20Reference))
  (if (< (Variables|Default|GetGracePeriod) 0.0)
    (CallFunction|Explode)))

(event EventTick
  (params (DeltaSeconds :type Float%20%28single-precision%29))
  ;[1 1 1] Update the velocity based on gravity
  (Variables|Default|SetGracePeriod (- (Variables|Default|GetGracePeriod) DeltaSeconds))
  (bind _output_get (Variables|Default|SetVelocityTracker (Math|Vector|MakeVector (.X (Math|Vector|BreakVector (Variables|Default|GetVelocityTracker))) (.Y (Math|Vector|BreakVector (Variables|Default|GetVelocityTracker))) (+ (.Z (Math|Vector|BreakVector (Variables|Default|GetVelocityTracker))) (* DeltaSeconds (Variables|Default|GetGravity))))))
  ;[1 1 1] Update the location based on velocity
  (bind _output_get_2 (Variables|Default|SetLocation (+ (* _output_get DeltaSeconds) (Variables|Default|GetLocation))))
  (Transformation|SetActorLocation self _output_get_2 false false))

(fn ConstructionScript)

(fn Initialize
  (Variables|Default|SetLocation (Transformation|GetActorLocation)))

(fn Explode
  (Variables|Default|SetGracePeriod 1e+01)
  ;[1 1 1] spawn sound effect - skye
  (Audio|SpawnSoundatLocation "/Game/SKYE/Audio/Bishop/Cue_BishopSplash.Cue_BishopSplash" (Transformation|GetActorLocation) "0, 0, 0" 1.0 1.0 0.0 0 0)
  (Actor|DestroyActor))